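; House2_BP is a destructible house actor that reacts when its DestructibleComponent fractures.
; On fracture it passes the Sphere's world location as a transform to RandomOrb's Ondestructbreak, then turns off the destructible's collision.
; It prints a debug string and destroys itself after a short delay, leaving a second, unconnected print-delay-destroy chain unused.
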(event `self.DestructibleComponent.OnComponentFracture`
  (params (HitPoint :type "Object.Vector Structure (by ref)") (HitDirection :type "Object.Vector Structure (by ref)"))
  (`/Game/Blueprints/RandomOrb.Ondestructbreak` (`self.RandomOrb`) (`KismetMathLibrary.MakeTransform` (`SceneComponent.K2_GetComponentLocation` (`self.Sphere`)) (struct) (1.0 1.0 1.0)))
  (`PrimitiveComponent.SetCollisionEnabled` (`self.DestructibleComponent`) "NoCollision")
  (`KismetSystemLibrary.PrintString` "Hello")
  (`KismetSystemLibrary.Delay` 2.5)
  (`self.K2_DestroyActor`))

(event `self.ReceiveBeginPlay`)

(event `self.ReceiveActorBeginOverlap`
  (params (OtherActor :type "Actor Object Reference")))

(event `self.ReceiveTick`
  (params (DeltaSeconds :type "Float (single-precision)")))

(fn `UserConstructionScript`)