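; Falling branch hazard for the forest boss's attacks that damages whatever it hits.
; The construction script randomly picks one of two branch meshes and gives it a random spin through its RotatingMovement component.
; On hit it applies damage scaled by the boss's DamageModifier, read from the game mode's boss reference, then plays a sound, disables collision and expires a few seconds later.
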(event `self.ReceiveBeginPlay`
  (bind _asmy_game (cast `/Game/Blueprints/MyGame` (`GameplayStatics.GetGameMode`)))
  (bind _asai_boss_1 (cast `/Game/Blueprints/ai/AI_Boss1` (`/Game/Blueprints/MyGame.Boss Ref` _asmy_game))))

(event `self.ReceiveHit`
  (params (MyComp :type "PrimitiveComponent Object Reference") (Other :type "Actor Object Reference") (OtherComp :type "PrimitiveComponent Object Reference") (bSelfMoved :type Boolean) (HitLocation :type "Object.Vector Structure") (HitNormal :type "Object.Vector Structure") (NormalImpulse :type "Object.Vector Structure") (Hit :type "EngineTypes.HitResult Structure (by ref)"))
  ;[1 1 1] Assign Projectile Vars (Based off Bow)
  (`GameplayStatics.ApplyDamage` Other (* (+ (/ (`/Game/Blueprints/ai/AI_Boss1.Damage Modifier` (stale `self.ReceiveBeginPlay` _asai_boss_1)) 5.0) 1.0) (`self.Base_Damageprojectile`)) null self)
  (`GameplayStatics.PlaySoundAtLocation` "/Game/StarterContent/Audio/Fire01_Cue.Fire01_Cue" HitLocation)
  (`PrimitiveComponent.SetCollisionEnabled` "NoCollision")
  (`self.SetLifeSpan` 4.0))

(event `self.ReceiveActorBeginOverlap`
  (params (OtherActor :type "Actor Object Reference")))

(event `self.ReceiveTick`
  (params (DeltaSeconds :type "Float (single-precision)")))

(fn `UserConstructionScript`
  (switch `int` (`KismetMathLibrary.RandomIntegerInRange` 0 1)
    (:`0`
      (`StaticMeshComponent.SetStaticMesh` "/Game/Meshes/NewForestBranch1.NewForestBranch1"))
    (:`1`
      (`StaticMeshComponent.SetStaticMesh` "/Game/Meshes/NewForestBranch2.NewForestBranch2")))
  (set `RotatingMovementComponent.RotationRate` (`KismetMathLibrary.MakeRot` (`KismetMathLibrary.RandomFloatInRange` -180.0 180.0) (`KismetMathLibrary.RandomFloatInRange` -180.0 180.0) (`KismetMathLibrary.RandomFloatInRange` -180.0 180.0)) (`self.RotatingMovement`)))