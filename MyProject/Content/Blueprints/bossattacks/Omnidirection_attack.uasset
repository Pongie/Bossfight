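; Spawner for the AI_Boss1 omnidirectional attack, firing volleys of Omnidirectionattack actors from the boss's transform.
; BeginPlay finds the boss and starts a looping timer whose random interval is rolled once.
; Each tick destroys the spawner if the boss is dead, otherwise a random pattern picks one to three delayed eight-actor volleys, later ones offset by variation vectors.
; The largest pattern loops back to repeat the three-volley sequence, giving six.
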(event `self.ReceiveBeginPlay`
  ;[1 1 1] init
  (bind _outactors (`GameplayStatics.GetAllActorsOfClass` "/Game/Blueprints/ai/AI_Boss1.AI_Boss1_C"))
  (bind _asai_boss_1 (cast `/Game/Blueprints/ai/AI_Boss1` (`KismetArrayLibrary.Array_Get` _outactors)))
  (set `self.BossRef` _asai_boss_1)
  (`KismetSystemLibrary.K2_SetTimer` null "OmniDirection" (`KismetMathLibrary.RandomFloatInRange` 15.0 30.0) true))

(event `OmniDirection`
  (bind _bossref (`self.BossRef`))
  (bind _omnidirectionattack (`self.omnidirectionattack`))
  (bind _pattern_ (`self.Pattern#`))
  (bind _set2variation (`self.set2variation`))
  (bind _set3variation (`self.set3variation`))
  (bind _rotation (.rotation (`SceneComponent.K2_GetComponentToWorld` _bossref)))
  (bind _rotation_2 (.rotation (`SceneComponent.K2_GetComponentToWorld` _bossref)))
  (bind _rotation_3 (.rotation (`SceneComponent.K2_GetComponentToWorld` _bossref)))
  (bind _rotation_4 (.rotation (`SceneComponent.K2_GetComponentToWorld` _bossref)))
  (bind _rotation_5 (.rotation (`SceneComponent.K2_GetComponentToWorld` _bossref)))
  (bind _rotation_6 (.rotation (`SceneComponent.K2_GetComponentToWorld` _bossref)))
  (bind _rotation_7 (.rotation (`SceneComponent.K2_GetComponentToWorld` _bossref)))
  (bind _rotation_8 (.rotation (`SceneComponent.K2_GetComponentToWorld` _bossref)))
  (bind _rotation_9 (.rotation (`SceneComponent.K2_GetComponentToWorld` _bossref)))
  (bind _rotation_10 (.rotation (`SceneComponent.K2_GetComponentToWorld` _bossref)))
  (bind _rotation_11 (.rotation (`SceneComponent.K2_GetComponentToWorld` _bossref)))
  (bind _rotation_12 (.rotation (`SceneComponent.K2_GetComponentToWorld` _bossref)))
  (bind _rotation_13 (.rotation (`SceneComponent.K2_GetComponentToWorld` _bossref)))
  (bind _rotation_14 (.rotation (`SceneComponent.K2_GetComponentToWorld` _bossref)))
  (bind _rotation_15 (.rotation (`SceneComponent.K2_GetComponentToWorld` _bossref)))
  (bind _rotation_16 (.rotation (`SceneComponent.K2_GetComponentToWorld` _bossref)))
  ;[1 1 1] cleanup
  (if (<= (`/Game/Blueprints/ai/AI_Boss1.Hitpoints` (`self.BossRef`)) 0.0)
    (`self.K2_DestroyActor`)
    (else
      (bind _output_get (set `self.Pattern#` (`KismetMathLibrary.RandomIntegerInRange` 0 3)))
      (switch `int` _output_get
        (:`Default`
          ;[1 1 1] spawn
          (`|SpawnActorFromClass` _omnidirectionattack (`SceneComponent.K2_GetComponentToWorld` _bossref) true :!label _label)
          (`|SpawnActorFromClass` _omnidirectionattack (`SceneComponent.K2_GetComponentToWorld` _bossref) true)
          (`|SpawnActorFromClass` _omnidirectionattack (`SceneComponent.K2_GetComponentToWorld` _bossref) true)
          (`|SpawnActorFromClass` _omnidirectionattack (`SceneComponent.K2_GetComponentToWorld` _bossref) true)
          (`|SpawnActorFromClass` _omnidirectionattack (`SceneComponent.K2_GetComponentToWorld` _bossref) true)
          (`|SpawnActorFromClass` _omnidirectionattack (`SceneComponent.K2_GetComponentToWorld` _bossref) true)
          (`|SpawnActorFromClass` _omnidirectionattack (`SceneComponent.K2_GetComponentToWorld` _bossref) true)
          (`|SpawnActorFromClass` _omnidirectionattack (`SceneComponent.K2_GetComponentToWorld` _bossref) true)
          (if (or (== (`self.Pattern#`) 1) (== (`self.Pattern#`) 2) (== (`self.Pattern#`) 3))
            (`KismetSystemLibrary.Delay` 0.5)
            (`|SpawnActorFromClass` _omnidirectionattack (`KismetMathLibrary.MakeTransform` (+ (.location (`SceneComponent.K2_GetComponentToWorld` _bossref)) (- (`KismetMathLibrary.Conv_RotatorToVector` _rotation_2) _set2variation)) _rotation_2 (.scale (`SceneComponent.K2_GetComponentToWorld` _bossref))) true)
            (`|SpawnActorFromClass` _omnidirectionattack (`KismetMathLibrary.MakeTransform` (+ (.location (`SceneComponent.K2_GetComponentToWorld` _bossref)) (- (`KismetMathLibrary.Conv_RotatorToVector` _rotation_3) _set2variation)) _rotation_3 (.scale (`SceneComponent.K2_GetComponentToWorld` _bossref))) true)
            (`|SpawnActorFromClass` _omnidirectionattack (`KismetMathLibrary.MakeTransform` (+ (.location (`SceneComponent.K2_GetComponentToWorld` _bossref)) (- (`KismetMathLibrary.Conv_RotatorToVector` _rotation_4) _set2variation)) _rotation_4 (.scale (`SceneComponent.K2_GetComponentToWorld` _bossref))) true)
            (`|SpawnActorFromClass` _omnidirectionattack (`KismetMathLibrary.MakeTransform` (+ (.location (`SceneComponent.K2_GetComponentToWorld` _bossref)) (- (`KismetMathLibrary.Conv_RotatorToVector` _rotation_5) _set2variation)) _rotation_5 (.scale (`SceneComponent.K2_GetComponentToWorld` _bossref))) true)
            (`|SpawnActorFromClass` _omnidirectionattack (`KismetMathLibrary.MakeTransform` (+ (.location (`SceneComponent.K2_GetComponentToWorld` _bossref)) (- (`KismetMathLibrary.Conv_RotatorToVector` _rotation_6) _set2variation)) _rotation_6 (.scale (`SceneComponent.K2_GetComponentToWorld` _bossref))) true)
            (`|SpawnActorFromClass` _omnidirectionattack (`KismetMathLibrary.MakeTransform` (+ (.location (`SceneComponent.K2_GetComponentToWorld` _bossref)) (- (`KismetMathLibrary.Conv_RotatorToVector` _rotation_7) _set2variation)) _rotation_7 (.scale (`SceneComponent.K2_GetComponentToWorld` _bossref))) true)
            (`|SpawnActorFromClass` _omnidirectionattack (`KismetMathLibrary.MakeTransform` (+ (.location (`SceneComponent.K2_GetComponentToWorld` _bossref)) (- (`KismetMathLibrary.Conv_RotatorToVector` _rotation_8) _set2variation)) _rotation_8 (.scale (`SceneComponent.K2_GetComponentToWorld` _bossref))) true)
            (`|SpawnActorFromClass` _omnidirectionattack (`KismetMathLibrary.MakeTransform` (+ (.location (`SceneComponent.K2_GetComponentToWorld` _bossref)) (- (`KismetMathLibrary.Conv_RotatorToVector` _rotation_9) _set2variation)) _rotation_9 (.scale (`SceneComponent.K2_GetComponentToWorld` _bossref))) true)
            (if (or false (== _pattern_ 2) (== _pattern_ 3))
              (`KismetSystemLibrary.Delay` 0.5)
              (`|SpawnActorFromClass` _omnidirectionattack (`KismetMathLibrary.MakeTransform` (+ (.location (`SceneComponent.K2_GetComponentToWorld` _bossref)) (- (`KismetMathLibrary.Conv_RotatorToVector` _rotation_10) _set3variation)) _rotation_10 (.scale (`SceneComponent.K2_GetComponentToWorld` _bossref))) true)
              (`|SpawnActorFromClass` _omnidirectionattack (`KismetMathLibrary.MakeTransform` (+ (.location (`SceneComponent.K2_GetComponentToWorld` _bossref)) (- (`KismetMathLibrary.Conv_RotatorToVector` _rotation_11) _set3variation)) _rotation_11 (.scale (`SceneComponent.K2_GetComponentToWorld` _bossref))) true)
              (`|SpawnActorFromClass` _omnidirectionattack (`KismetMathLibrary.MakeTransform` (+ (.location (`SceneComponent.K2_GetComponentToWorld` _bossref)) (- (`KismetMathLibrary.Conv_RotatorToVector` _rotation_12) _set3variation)) _rotation_12 (.scale (`SceneComponent.K2_GetComponentToWorld` _bossref))) true)
              (`|SpawnActorFromClass` _omnidirectionattack (`KismetMathLibrary.MakeTransform` (+ (.location (`SceneComponent.K2_GetComponentToWorld` _bossref)) (- (`KismetMathLibrary.Conv_RotatorToVector` _rotation_13) _set3variation)) _rotation_13 (.scale (`SceneComponent.K2_GetComponentToWorld` _bossref))) true)
              (`|SpawnActorFromClass` _omnidirectionattack (`KismetMathLibrary.MakeTransform` (+ (.location (`SceneComponent.K2_GetComponentToWorld` _bossref)) (- (`KismetMathLibrary.Conv_RotatorToVector` _rotation_14) _set3variation)) _rotation_14 (.scale (`SceneComponent.K2_GetComponentToWorld` _bossref))) true)
              (`|SpawnActorFromClass` _omnidirectionattack (`KismetMathLibrary.MakeTransform` (+ (.location (`SceneComponent.K2_GetComponentToWorld` _bossref)) (- (`KismetMathLibrary.Conv_RotatorToVector` _rotation_15) _set3variation)) _rotation_15 (.scale (`SceneComponent.K2_GetComponentToWorld` _bossref))) true)
              (`|SpawnActorFromClass` _omnidirectionattack (`KismetMathLibrary.MakeTransform` (+ (.location (`SceneComponent.K2_GetComponentToWorld` _bossref)) (- (`KismetMathLibrary.Conv_RotatorToVector` _rotation_16) _set3variation)) _rotation_16 (.scale (`SceneComponent.K2_GetComponentToWorld` _bossref))) true)
              (`|SpawnActorFromClass` _omnidirectionattack (`KismetMathLibrary.MakeTransform` (+ (.location (`SceneComponent.K2_GetComponentToWorld` _bossref)) (- (`KismetMathLibrary.Conv_RotatorToVector` _rotation) _set3variation)) _rotation (.scale (`SceneComponent.K2_GetComponentToWorld` _bossref))) true)
              (if (== (`self.Pattern#`) 3)
                (set `self.Pattern#` 2)
                (`KismetSystemLibrary.Delay` 0.5 :!label _label_2)
                (goto _label)))))
        (:`0`
          (goto _label_2))
        (:`1`
          (goto _label_2))
        (:`2`
          (goto _label_2))
        (:`3`
          (goto _label_2))))))

(fn `UserConstructionScript`)