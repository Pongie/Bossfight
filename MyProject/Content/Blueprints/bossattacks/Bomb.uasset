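; Bomb actor for boss attacks that lights a fuse when first damaged, then explodes with radial damage.
; Once hit, it damages itself every Tick until Health runs out, so further hits shorten the fuse.
; The explosion spawns an emitter, scales its damage by the AI_Boss1 DamageModifier taken from MyGame, and destroys the actor.
; The construction script sizes a sphere to preview the explosion radius.
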(event `self.ReceiveBeginPlay`
  (bind _asmy_game (cast `/Game/Blueprints/MyGame` (`GameplayStatics.GetGameMode`)))
  (bind _asai_boss_1 (cast `/Game/Blueprints/ai/AI_Boss1` (`/Game/Blueprints/MyGame.Boss Ref` _asmy_game))))

(event `self.ReceiveTick`
  (params (DeltaSeconds :type "Float (single-precision)"))
  ;[1 1 1] Apply Damage Over time to bomb  if hit
  (if (`self.bhasbeendamaged`)
    (`GameplayStatics.ApplyDamage` self (* (`self.Damageovertime`) DeltaSeconds) null self)))

(event `self.ReceiveAnyDamage`
  (params (Damage :type "Float (single-precision)") (DamageType :type "DamageType Object Reference") (InstigatedBy :type "Controller Object Reference") (DamageCauser :type "Actor Object Reference"))
  (bind _returnvalue (`self.K2_GetActorLocation`))
  (`|ExecutionSequence`
    (:`then_0`
      ;[1 1 1] Spawn Fuse particle effect
      (if (not (`self.bhasbeendamaged`))
        (`ActorComponent.Activate` (`self.ParticleSystem`) false)
        (set `self.bhasbeendamaged` true)))
    (:`then_1`
      (if (not (`self.hasExploded`))
        ;[1 1 1] Apply Damage/Kill
        (bind _output_get (set `self.health` (- (`self.health`) Damage)))
        (if (<= _output_get 0.0)
          (set `self.hasExploded` true)
          (`GameplayStatics.SpawnEmitterAtLocation` "/Game/StarterContent/Particles/P_Explosion.P_Explosion" _returnvalue)
          (`GameplayStatics.ApplyRadialDamage` :`BaseDamage` (* (+ (/ (`/Game/Blueprints/ai/AI_Boss1.Damage Modifier` (stale `self.ReceiveBeginPlay` _asai_boss_1)) 5.0) 1.0) (`self.ExplosionDamage`)) :`Origin` _returnvalue :`DamageRadius` (`self.ExplosionRadius`) :`bDoFullDamage` true)
          (`self.K2_DestroyActor`))))))

(event `self.ReceiveActorBeginOverlap`
  (params (OtherActor :type "Actor Object Reference")))

(fn `UserConstructionScript`
  (`SphereComponent.SetSphereRadius` (`self.ExplosionRadiusView`) (`self.ExplosionRadius`) true))