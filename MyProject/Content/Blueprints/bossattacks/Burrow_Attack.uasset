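; Boss burrow attack actor that damages and knocks back what it hits, then repositions the boss where it ends.
; Hits pass through a DoOnce that a looping timer resets, throttling damage and collapse sound.
; Player characters are launched along a blend of actor forward and impact normal with some lift.
; A short kill timer moves the boss to the actor's XY and rotation, keeping its height, then destroys the actor.
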(event `self.ReceiveBeginPlay`
  (`KismetSystemLibrary.K2_SetTimer` null "BurrowTick" 0.1 true)
  (`KismetSystemLibrary.K2_SetTimer` null "KillTimer" 1.7))

(event `BurrowTick`
  ;[1 1 1] Damage/Knockback
  (goto _label :!via `Reset`))

(event `self.ReceiveHit`
  (params (MyComp :type "PrimitiveComponent Object Reference") (Other :type "Actor Object Reference") (OtherComp :type "PrimitiveComponent Object Reference") (bSelfMoved :type Boolean) (HitLocation :type "Object.Vector Structure") (HitNormal :type "Object.Vector Structure") (NormalImpulse :type "Object.Vector Structure") (Hit :type "EngineTypes.HitResult Structure (by ref)"))
  ;[1 1 1] Damage/Knockback
  (`/Engine/EditorBlueprintResources/StandardMacros.DoOnce` false :!label _label
    (:`Completed`
      (`GameplayStatics.ApplyDamage` Other (`self.Base_Damageprojectile`) null self)
      (`GameplayStatics.PlaySoundAtLocation` "/Game/StarterContent/Audio/Collapse_Cue.Collapse_Cue" HitLocation)
      (bind _asmy_character (cast `/Game/Blueprints/MyCharacter` Other))
      (`Character.LaunchCharacter` _asmy_character (* (`KismetMathLibrary.MakeVector` (.x (`KismetMathLibrary.VLerp` (`KismetMathLibrary.GetForwardVector` (`self.K2_GetActorRotation`)) (`.ImpactNormal` (`GameplayStatics.BreakHitResult` Hit)) 0.5)) (.y (`KismetMathLibrary.VLerp` (`KismetMathLibrary.GetForwardVector` (`self.K2_GetActorRotation`)) (`.ImpactNormal` (`GameplayStatics.BreakHitResult` Hit)) 0.5)) 0.25) 1555.0) true true))))

(event `self.ReceiveActorBeginOverlap`
  (params (OtherActor :type "Actor Object Reference")))

(event `self.ReceiveTick`
  (params (DeltaSeconds :type "Float (single-precision)")))

(event `KillTimer`
  (bind _bossref (`self.bossRef`))
  ;[1 1 1] Dynamic  Destroyed
  (`self.SetActorRotation` _bossref (.rotation (`self.GetTransform`)))
  (`self.K2_SetActorLocation` _bossref (`KismetMathLibrary.MakeVector` (.x (.location (`self.GetTransform`))) (.y (.location (`self.GetTransform`))) (.z (`self.K2_GetActorLocation` _bossref))) false)
  (`self.K2_DestroyActor`))

(fn `UserConstructionScript`)