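; Bouncing boss-attack projectile that deals damage with a lightning flash and sound on every hit.
; Hitting one of up to four player characters disables collision and destroys it after a delay; other hits leave it active.
; On each bounce, a large sphere trace between fixed coordinates, independent of the projectile's position, sets the hit component as the ProjectileMovement homing target.
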(event `self.ReceiveBeginPlay`
  (cast `/Game/Blueprints/MyGame` (`GameplayStatics.GetGameMode`)))

(event `self.ReceiveHit`
  (params (MyComp :type "PrimitiveComponent Object Reference") (Other :type "Actor Object Reference") (OtherComp :type "PrimitiveComponent Object Reference") (bSelfMoved :type Boolean) (HitLocation :type "Object.Vector Structure") (HitNormal :type "Object.Vector Structure") (NormalImpulse :type "Object.Vector Structure") (Hit :type "EngineTypes.HitResult Structure (by ref)"))
  (bind (_bblockinghit _time _location _normal _impactpoint _impactnormal _physmat _hitactor) (`GameplayStatics.BreakHitResult` Hit))
  (bind _base_damageprojectile (`self.Base_Damageprojectile`))
  ;[1 1 1] Assign Projectile Vars (Based off Bow)
  (if (or (== _hitactor (`GameplayStatics.GetPlayerCharacter` 0)) (== (`GameplayStatics.GetPlayerCharacter` 1) _hitactor) (== (`GameplayStatics.GetPlayerCharacter` 2) _hitactor) (== (`GameplayStatics.GetPlayerCharacter` 3) _hitactor))
    (`GameplayStatics.ApplyDamage` Other _base_damageprojectile null self)
    (bind _returnvalue (`GameplayStatics.SpawnEmitterAtLocation` "/Game/Outsourced/Effects/premade/lightningflash.lightningflash" HitLocation))
    (`GameplayStatics.PlaySoundAtLocation` "/Game/Sounds/sword_attack.sword_attack" HitLocation)
    (`PrimitiveComponent.SetCollisionEnabled` "NoCollision")
    (`KismetSystemLibrary.Delay` 0.6)
    (`ActorComponent.K2_DestroyComponent` _returnvalue)
    (`KismetSystemLibrary.Delay` 1.42)
    (`self.K2_DestroyActor`)
    (else
      (`GameplayStatics.ApplyDamage` Other _base_damageprojectile null self)
      (bind _returnvalue_2 (`GameplayStatics.SpawnEmitterAtLocation` "/Game/Outsourced/Effects/premade/lightningflash.lightningflash" HitLocation))
      (`GameplayStatics.PlaySoundAtLocation` "/Game/Sounds/sword_attack.sword_attack" HitLocation)
      (`KismetSystemLibrary.Delay` 0.2)
      (`ActorComponent.K2_DestroyComponent` _returnvalue_2))))

(event `self.ReceiveActorBeginOverlap`
  (params (OtherActor :type "Actor Object Reference")))

(event `self.ReceiveTick`
  (params (DeltaSeconds :type "Float (single-precision)")))

(event `self.ProjectileMovement.OnProjectileBounce`
  (params (ImpactResult :type "EngineTypes.HitResult Structure (by ref)") (ImpactVelocity :type "Object.Vector Structure (by ref)"))
  (bind _outhit (`KismetSystemLibrary.SphereTraceSingle_NEW` (11111.0 11111.0 111.0) (-11111.0 -11111.0 -111.0) 1111.0 "TraceTypeQuery1"))
  (set `ProjectileMovementComponent.HomingTargetComponent` (`.HitComponent` (`GameplayStatics.BreakHitResult` _outhit)) (`self.ProjectileMovement`)))

(fn `UserConstructionScript`)