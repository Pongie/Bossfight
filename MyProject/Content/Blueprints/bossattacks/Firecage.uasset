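; Firecage is a destructible fire hazard actor, filed under boss attacks, that damages whatever it hits.
; Hit events apply ContactDamage to the other actor and play a fire cue at the world origin.
; Any damage received removes one Health point regardless of amount, destroying the actor at zero.
; The construction script sizes the ExplosionRadiusView sphere from ExplosionRadius, though no explosion logic uses it here.
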(event `self.ReceiveAnyDamage`
  (params (Damage :type "Float (single-precision)") (DamageType :type "DamageType Object Reference") (InstigatedBy :type "Controller Object Reference") (DamageCauser :type "Actor Object Reference"))
  (bind _output_get (set `self.health` (- (`self.health`) 1.0)))
  (if (<= _output_get 0.0)
    (`self.K2_DestroyActor`)))

(event `self.ReceiveHit`
  (params (MyComp :type "PrimitiveComponent Object Reference") (Other :type "Actor Object Reference") (OtherComp :type "PrimitiveComponent Object Reference") (bSelfMoved :type Boolean) (HitLocation :type "Object.Vector Structure") (HitNormal :type "Object.Vector Structure") (NormalImpulse :type "Object.Vector Structure") (Hit :type "EngineTypes.HitResult Structure (by ref)"))
  (`GameplayStatics.ApplyDamage` Other (`self.contactDamage`) null self)
  (`GameplayStatics.PlaySoundAtLocation` "/Game/StarterContent/Audio/Fire01_Cue.Fire01_Cue"))

(event `self.ReceiveBeginPlay`)

(event `self.ReceiveActorBeginOverlap`
  (params (OtherActor :type "Actor Object Reference")))

(fn `UserConstructionScript`
  (`SphereComponent.SetSphereRadius` (`self.ExplosionRadiusView`) (`self.ExplosionRadius`) true))