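; Boss-attack tornado character that wanders the level and launches any MyCharacter it touches along its forward vector with added lift.
; A looping timer and Targetpoint overlaps randomly change the current index into the TargetPoint_bp actors.
; Tick steps it along that point's normalized world location, used as a direction rather than an offset from the tornado.
; Overlapping Nadobounds actors toggles Flip, which negates that direction's X and Y.
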(event `swapPosition`
  (bind _currentwaypoint (`self.Currentwaypoint`))
  ;[1 1 1] random swap between positions
  (if (>= (`KismetMathLibrary.RandomFloatInRange` 0.0 100.0) 50.0)
    (set `self.Currentwaypoint` (- (`self.Currentwaypoint`) (`KismetMathLibrary.RandomIntegerInRange` 1 4)))
    (else
      (set `self.Currentwaypoint` (+ (`self.Currentwaypoint`) (`KismetMathLibrary.RandomIntegerInRange` 1 4)))))
  (if (or (>= _currentwaypoint 10) (<= _currentwaypoint -1))
    (if (!= (`self.Currentwaypoint`) 5)
      (set `self.Currentwaypoint` 5)
      (else
        (set `self.Currentwaypoint` (`KismetMathLibrary.RandomIntegerInRange` 0 4)))))
  (`self.K2_SetActorTransform` (`KismetMathLibrary.MakeTransform` (+ (* (`KismetMathLibrary.Normal` (`self.K2_GetActorLocation` (`KismetArrayLibrary.Array_Get` (`self.Waypoints`) (`self.Currentwaypoint`)))) (* (`GameplayStatics.GetWorldDeltaSeconds`) (`CharacterMovementComponent.MaxWalkSpeed` (`self.CharacterMovement`)))) (.location (`SceneComponent.K2_GetComponentToWorld` (`self.Mesh`)))) (`KismetMathLibrary.Conv_VectorToRotator` (`KismetMathLibrary.GetForwardVector` (.rotation (`SceneComponent.K2_GetComponentToWorld` (`self.Mesh`))))) (.scale (`SceneComponent.K2_GetComponentToWorld` (`self.Mesh`))))))

(event `self.ReceiveBeginPlay`
  ;[1 1 1] init
  (bind _outactors (`GameplayStatics.GetAllActorsOfClass` "/Game/Blueprints/TargetPoint_bp.TargetPoint_bp_C"))
  (set `self.Waypoints` _outactors)
  (`KismetSystemLibrary.K2_SetTimer` null "swapPosition" (`KismetMathLibrary.RandomFloatInRange` 2.5 20.0) true)
  (if (== (`KismetMathLibrary.RandomIntegerInRange` 0 8) (`self.Currentwaypoint`))
    (if (!= (`self.Currentwaypoint`) 5)
      (set `self.Currentwaypoint` 5)
      (else
        (set `self.Currentwaypoint` (`KismetMathLibrary.RandomIntegerInRange` 0 4))))
    (else
      (set `self.Currentwaypoint` 0)))
  (`self.K2_SetActorTransform` (`KismetMathLibrary.MakeTransform` (+ (* (`KismetMathLibrary.Normal` (`self.K2_GetActorLocation` (`KismetArrayLibrary.Array_Get` (`self.Waypoints`) (`self.Currentwaypoint`)))) (* (`GameplayStatics.GetWorldDeltaSeconds`) (`CharacterMovementComponent.MaxWalkSpeed` (`self.CharacterMovement`)))) (.location (`SceneComponent.K2_GetComponentToWorld` (`self.Mesh`)))) (`KismetMathLibrary.Conv_VectorToRotator` (`KismetMathLibrary.GetForwardVector` (.rotation (`SceneComponent.K2_GetComponentToWorld` (`self.Mesh`))))) (.scale (`SceneComponent.K2_GetComponentToWorld` (`self.Mesh`))))))

(event `self.ReceiveActorBeginOverlap`
  (params (OtherActor :type "Actor Object Reference"))
  ;[1 1 1] tornado impulse
  (bind _asmy_character (cast `/Game/Blueprints/MyCharacter` OtherActor)
    (:`then`
      (`self.LaunchCharacter` (stale `self.ReceiveHit` _asmy_character) (`KismetMathLibrary.MakeVector` (.x (* (`KismetMathLibrary.GetForwardVector` (`self.K2_GetActorRotation`)) 350.0)) (.y (* (`KismetMathLibrary.GetForwardVector` (`self.K2_GetActorRotation`)) 350.0)) (+ (.z (* (`KismetMathLibrary.GetForwardVector` (`self.K2_GetActorRotation`)) 350.0)) 100.0)) true false :!label _label)
      (`self.LaunchCharacter` _asmy_character (`KismetMathLibrary.MakeVector` (.x (* (`KismetMathLibrary.GetForwardVector` (`self.K2_GetActorRotation`)) 350.0)) (.y (* (`KismetMathLibrary.GetForwardVector` (`self.K2_GetActorRotation`)) 350.0)) (+ (.z (* (`KismetMathLibrary.GetForwardVector` (`self.K2_GetActorRotation`)) 350.0)) 100.0)) true false))
    (:`CastFailed`
      (if (`self.ActorHasTag` OtherActor "Nadobounds")
        (`/Engine/EditorBlueprintResources/StandardMacros.FlipFlop`
          (:`A`
            (set `self.flip` true))
          (:`B`
            (set `self.flip` false)))))))

(event `self.ReceiveHit`
  (params (MyComp :type "PrimitiveComponent Object Reference") (Other :type "Actor Object Reference") (OtherComp :type "PrimitiveComponent Object Reference") (bSelfMoved :type Boolean) (HitLocation :type "Object.Vector Structure") (HitNormal :type "Object.Vector Structure") (NormalImpulse :type "Object.Vector Structure") (Hit :type "EngineTypes.HitResult Structure (by ref)"))
  ;[1 1 1] tornado impulse
  (bind _asmy_character (cast `/Game/Blueprints/MyCharacter` Other))
  (goto _label))

(event `self.CapsuleComponent.OnComponentBeginOverlap`
  (params (OtherActor :type "Actor Object Reference") (OtherComp :type "PrimitiveComponent Object Reference") (OtherBodyIndex :type Integer) (bFromSweep :type Boolean) (SweepResult :type "EngineTypes.HitResult Structure (by ref)"))
  (bind _returnvalue (`KismetMathLibrary.RandomIntegerInRange` 0 8))
  ;[1 1 1] tornado movement
  (if (`self.ActorHasTag` OtherActor "Targetpoint")
    (if (== _returnvalue (`self.Currentwaypoint`))
      (if (!= (`self.Currentwaypoint`) 5)
        (set `self.Currentwaypoint` 5)
        (else
          (set `self.Currentwaypoint` (`KismetMathLibrary.RandomIntegerInRange` 0 4))))
      (`self.K2_SetActorTransform` (`KismetMathLibrary.MakeTransform` (+ (* (`KismetMathLibrary.Normal` (`self.K2_GetActorLocation` (`KismetArrayLibrary.Array_Get` (`self.Waypoints`) (`self.Currentwaypoint`)))) (* (`GameplayStatics.GetWorldDeltaSeconds`) (`CharacterMovementComponent.MaxWalkSpeed` (`self.CharacterMovement`)))) (.location (`SceneComponent.K2_GetComponentToWorld` (`self.Mesh`)))) (`KismetMathLibrary.Conv_VectorToRotator` (`KismetMathLibrary.GetForwardVector` (.rotation (`SceneComponent.K2_GetComponentToWorld` (`self.Mesh`))))) (.scale (`SceneComponent.K2_GetComponentToWorld` (`self.Mesh`)))) :!label _label_2)
      (else
        (set `self.Currentwaypoint` _returnvalue)))))

(event `self.ReceiveTick`
  (params (DeltaSeconds :type "Float (single-precision)"))
  (bind _returnvalue (`self.K2_GetActorLocation` (`KismetArrayLibrary.Array_Get` (`self.Waypoints`) (`self.Currentwaypoint`))))
  ;[1 1 1] tornado movement
  (if (`self.flip`)
    (`self.K2_SetActorTransform` (`KismetMathLibrary.MakeTransform` (+ (* (`KismetMathLibrary.Normal` (`KismetMathLibrary.MakeVector` (.x (- _returnvalue (* _returnvalue 2.0))) (.y (- _returnvalue (* _returnvalue 2.0))) (.z _returnvalue))) (* (`GameplayStatics.GetWorldDeltaSeconds`) (`CharacterMovementComponent.MaxWalkSpeed` (`self.CharacterMovement`)))) (.location (`SceneComponent.K2_GetComponentToWorld` (`self.Mesh`)))) (`KismetMathLibrary.Conv_VectorToRotator` (`KismetMathLibrary.GetForwardVector` (.rotation (`SceneComponent.K2_GetComponentToWorld` (`self.Mesh`))))) (.scale (`SceneComponent.K2_GetComponentToWorld` (`self.Mesh`)))))
    (else
      (goto _label_2))))

(fn `UserConstructionScript`)