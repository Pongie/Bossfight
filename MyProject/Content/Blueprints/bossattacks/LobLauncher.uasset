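; LobLauncher is a boss attack projectile that stops after a random delay, then rises and grows before launching a barrage.
; PerformAttack sphere-traces, fires homing LobAttack missiles at MyCharacter targets highlighted via custom depth, then scatters randomized LobAttack2 firework shots.
; An enraged boss may repeat the barrage with decreasing odds before the launcher destroys itself.
; Missile and cooldown-gated contact damage scale with the boss's DamageModifier.
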(event `PerformAttack`
  (bind _returnvalue (`self.K2_GetActorLocation`))
  (bind _returnvalue_2 (`SceneComponent.K2_GetComponentLocation`))
  (bind _homingtarget (`self.HomingTarget`))
  ;[1 1 1] Homing Missle
  (bind _outhits (`KismetSystemLibrary.SphereTraceMultiForObjects` _returnvalue_2 (+ (`KismetMathLibrary.MakeVector` (.x _returnvalue_2) (.y _returnvalue_2) (- (.z _returnvalue_2) 400.0)) (0.0 0.0 0.0)) 4444.0 (`|MakeArray` "ObjectTypeQuery7" :!type "EngineTypes.EObjectTypeQuery Enum") true))
  (bind _output_get (set `self.NumbofTargets` (- (`KismetArrayLibrary.Array_Length` _outhits) 1)))
  (for _ (range (+ (`KismetMathLibrary.RandomIntegerInRange` 8 13) 1)) :!label _label
    ;;[1 1 1] Taargeting for missle
    (bind _asmy_character (cast `/Game/Blueprints/MyCharacter` null))
    (`/Engine/EditorBlueprintResources/StandardMacros.IsValid` _homingtarget
      (:`Is Valid`
        (`PrimitiveComponent.SetRenderCustomDepth` _homingtarget false))
      (:`Is Not Valid`
        _))
    (bind _output_get_2 (set `self.HomingTarget` (`Character.CapsuleComponent` _asmy_character)))
    (`PrimitiveComponent.SetRenderCustomDepth` _homingtarget true)
    (`PrimitiveComponent.SetRenderCustomDepth` _output_get_2 true)
    (bind _returnvalue_3 (`|SpawnActorFromClass` "/Game/Blueprints/bossattacks/LobAttack.LobAttack_C" (`KismetMathLibrary.MakeTransform` (- _returnvalue (0.0 0.0 190.0)) (`KismetMathLibrary.MakeRot` 0.0 (.yaw (`KismetMathLibrary.FindLookAtRotation` _returnvalue (`self.K2_GetActorLocation` _asmy_character)))) (0.33 0.33 0.33)) true (`self.LocalBossRef`)))
    (set `/Game/Blueprints/bossattacks/LobAttack.damage` (+ (* (/ (`/Game/Blueprints/ai/AI_Boss1.Damage Modifier` (`self.LocalBossRef`)) 5.0) (`/Game/Blueprints/bossattacks/LobAttack.damage` _returnvalue_3)) 2.0) _returnvalue_3)
    (`/Game/Blueprints/bossattacks/LobAttack.Homing Missle2` _returnvalue_3 (`self.HomingTarget`)))
  ;[1 1 1] Firework Atk
  (for _ (range (+ (`KismetMathLibrary.RandomIntegerInRange` 8 18) 1))
    (`GameplayStatics.PlaySoundAtLocation` "/Game/Sounds/lob_attack_Cue.lob_attack_Cue")
    (bind _returnvalue_4 (`|SpawnActorFromClass` "/Game/Blueprints/bossattacks/LobAttack2.LobAttack2_C" (`KismetMathLibrary.MakeTransform` (.location (`self.GetTransform` self)) (`KismetMathLibrary.MakeRot` (.pitch (.rotation (`self.GetTransform` self))) (+ (.yaw (.rotation (`self.GetTransform` self))) (`KismetMathLibrary.RandomFloatInRange` -180.0 180.0)) (.roll (.rotation (`self.GetTransform` self)))) (0.33 0.33 0.33)) true (`self.LocalBossRef`)))
    (set `/Game/Blueprints/bossattacks/LobAttack2.damage` (+ (* (/ (`/Game/Blueprints/ai/AI_Boss1.Damage Modifier` (`self.LocalBossRef`)) 5.0) (`/Game/Blueprints/bossattacks/LobAttack2.damage` _returnvalue_4)) 2.0) _returnvalue_4)
    (bind _projectilemovement (`/Game/Blueprints/bossattacks/LobAttack2.ProjectileMovement` _returnvalue_4))
    (set `MovementComponent.Velocity` (- (`MovementComponent.Velocity` _projectilemovement) (`KismetMathLibrary.MakeVector` (`KismetMathLibrary.RandomFloatInRange` -110.0 111.0) (`KismetMathLibrary.RandomFloatInRange` -110.0 111.0) (`KismetMathLibrary.RandomFloatInRange` -110.0 111.0))) _projectilemovement)
    (set `ProjectileMovementComponent.ProjectileGravityScale` (`KismetMathLibrary.RandomFloatInRange` 0.5 4.0) _projectilemovement)
    (set `ProjectileMovementComponent.InitialSpeed` (* (`ProjectileMovementComponent.InitialSpeed` _projectilemovement) (`KismetMathLibrary.RandomFloatInRange` 0.5 1.5)) _projectilemovement))
  (if (`/Game/Blueprints/ai/AI_Boss1.enraged` (`self.LocalBossRef`))
    (if (>= (`KismetMathLibrary.RandomFloatInRange` 0.0 100.0) (`self.LoweringPercentile`))
      (set `self.LoweringPercentile` (+ (`self.LoweringPercentile`) 10.0))
      (goto _label)
      (else
        _)))
  (`self.K2_DestroyActor`))

(event `Float`
  (bind _projectilemovement (`self.ProjectileMovement`))
  ;[1 1 1] Stop Moving
  (set `ProjectileMovementComponent.MaxSpeed` 0.0 _projectilemovement)
  (set `MovementComponent.Velocity` (0.0 0.0 0.0) _projectilemovement)
  (`ProjectileMovementComponent.SetVelocityInLocalSpace` _projectilemovement (0.0 0.0 0.0))
  (set `self.MoveupGate` true)
  (set `self.RotationStart` true))

(event `self.ReceiveBeginPlay`
  ;[1 1 1] Init
  (bind _asmy_game (cast `/Game/Blueprints/MyGame` (`GameplayStatics.GetGameMode`)))
  (bind _asai_boss_1 (cast `/Game/Blueprints/ai/AI_Boss1` (`/Game/Blueprints/MyGame.Boss Ref` _asmy_game))
    (:`then`
      _)
    (:`CastFailed`
      _))
  (set `self.LocalBossRef` _asai_boss_1)
  (`KismetSystemLibrary.K2_SetTimer` null "Float" (`KismetMathLibrary.RandomFloatInRange` 0.2 3.5)))

(event `self.ReceiveHit`
  (params (MyComp :type "PrimitiveComponent Object Reference") (Other :type "Actor Object Reference") (OtherComp :type "PrimitiveComponent Object Reference") (bSelfMoved :type Boolean) (HitLocation :type "Object.Vector Structure") (HitNormal :type "Object.Vector Structure") (NormalImpulse :type "Object.Vector Structure") (Hit :type "EngineTypes.HitResult Structure (by ref)"))
  ;[1 1 1] If Hitting
  (`/Engine/EditorBlueprintResources/StandardMacros.CompareFloat` (`self.coolDown`) (`KismetSystemLibrary.GetGameTimeInSeconds`)
    (:`<`
      (`GameplayStatics.ApplyDamage` Other (* (+ (/ (`/Game/Blueprints/ai/AI_Boss1.Damage Modifier` (stale `self.ReceiveBeginPlay` _asai_boss_1)) 5.0) 2.0) (`self.Base_Damageprojectile`)) null self)
      (`GameplayStatics.PlaySoundAtLocation` "/Game/StarterContent/Audio/Fire01_Cue.Fire01_Cue" HitLocation)
      (set `self.coolDown` (+ (`KismetSystemLibrary.GetGameTimeInSeconds`) 0.25)))))

(event `self.ReceiveTick`
  (params (DeltaSeconds :type "Float (single-precision)"))
  ;[1 1 1] Float Attack
  (if (`self.RotationStart`)
    (`self.K2_SetActorTransform` (`KismetMathLibrary.MakeTransform` (`self.K2_GetActorLocation`) (* (`self.StartRot`) 2.0) (`self.GetActorScale3D`)))
    (if (`self.MoveupGate`)
      (bind _output_get (set `self.StartScale` (+ (`self.StartScale`) (0.15 0.15 0.15))))
      (`self.K2_SetActorTransform` (`KismetMathLibrary.MakeTransform` (+ (`self.K2_GetActorLocation`) (0.0 0.0 10.0)) (`self.K2_GetActorRotation`) _output_get))
      (set `self.Counter` (+ (`self.Counter`) 1))
      (if (== (`self.Counter`) 50)
        (`/Engine/EditorBlueprintResources/StandardMacros.DoOnce` false
          (:`Completed`
            (set `self.MoveupGate` false)
            (`self.PerformAttack`)))))))

(event `self.ReceiveActorBeginOverlap`
  (params (OtherActor :type "Actor Object Reference"))
  ;[1 1 1] If Hitting
)

(fn `UserConstructionScript`)