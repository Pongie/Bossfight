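; Homing projectile actor, filed under boss attacks, that damages whatever it hits.
; The HomingMissle event takes a target component and, if valid, turns on ProjectileMovement homing toward it.
; On Hit it applies damage, spawns impact particles and sound, disables collision, then destroys itself after a short delay.
; The Sphere's component-hit event only prints the hit actor's name.
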(event `self.ReceiveHit`
  (params (MyComp :type "PrimitiveComponent Object Reference") (Other :type "Actor Object Reference") (OtherComp :type "PrimitiveComponent Object Reference") (bSelfMoved :type Boolean) (HitLocation :type "Object.Vector Structure") (HitNormal :type "Object.Vector Structure") (NormalImpulse :type "Object.Vector Structure") (Hit :type "EngineTypes.HitResult Structure (by ref)"))
  ;[1 1 1] Assign Projectile Vars (Based off Bow)
  (`GameplayStatics.ApplyDamage` Other (`self.Base_Damageprojectile`) null self)
  (`GameplayStatics.SpawnEmitterAtLocation` "/Game/Blueprints/HitConveyance.HitConveyance" HitLocation)
  (`GameplayStatics.PlaySoundAtLocation` "/Game/StarterContent/Audio/Explosion02.Explosion02" HitLocation)
  (`PrimitiveComponent.SetCollisionEnabled` "NoCollision")
  (`KismetSystemLibrary.Delay` 1.0)
  (`self.K2_DestroyActor`))

(event `self.ReceiveBeginPlay`)

(event `self.ReceiveActorBeginOverlap`
  (params (OtherActor :type "Actor Object Reference")))

(event `self.ReceiveTick`
  (params (DeltaSeconds :type "Float (single-precision)")))

(event `self.Sphere.OnComponentHit`
  (params (OtherActor :type "Actor Object Reference") (OtherComp :type "PrimitiveComponent Object Reference") (NormalImpulse :type "Object.Vector Structure") (Hit :type "EngineTypes.HitResult Structure (by ref)"))
  (`KismetSystemLibrary.PrintString` (`KismetSystemLibrary.GetDisplayName` OtherActor)))

(event `Homing Missle`
  (params (TargetToHit :type "PrimitiveComponent Object Reference"))
  (bind _projectilemovement (`self.ProjectileMovement`))
  ;[1 1 1] Home
  (if (`KismetSystemLibrary.IsValid` TargetToHit)
    (set `ProjectileMovementComponent.HomingTargetComponent` TargetToHit _projectilemovement)
    (set `ProjectileMovementComponent.bIsHomingProjectile` true _projectilemovement)
    (set `ProjectileMovementComponent.HomingAccelerationMagnitude` 1000.0 _projectilemovement)))

(fn `UserConstructionScript`)