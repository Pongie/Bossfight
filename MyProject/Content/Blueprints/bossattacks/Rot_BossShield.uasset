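; Boss shield actor with four mesh segments that stays centered on the first AI_Boss1 found at BeginPlay, copying its location every Tick.
; Each segment has its own hit points, loses one per component hit regardless of source, and plays a sound.
; A depleted segment hides and drops collision, then a named timer restores its health, visibility and collision after 45 seconds.
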(event `self.ReceiveBeginPlay`
  (set `self.hitpointshield1` 3.0)
  (set `self.hitpointshield2` 3.0)
  (set `self.hitpointshield3` 3.0)
  (set `self.hitpointshield4` 3.0)
  (bind _outactors (`GameplayStatics.GetAllActorsOfClass` "/Game/Blueprints/ai/AI_Boss1.AI_Boss1_C"))
  (bind _asai_boss_1 (cast `/Game/Blueprints/ai/AI_Boss1` (`KismetArrayLibrary.Array_Get` _outactors)))
  (set `self.BossRef` _asai_boss_1))

(event `self.ReceiveTick`
  (params (DeltaSeconds :type "Float (single-precision)"))
  (`self.K2_SetActorLocation` (.location (`self.GetTransform` (`self.BossRef`))))
  (if (== (`self.BossRef`) null)
    _))

(event `self.StaticMesh.OnComponentHit`
  (params (OtherActor :type "Actor Object Reference") (OtherComp :type "PrimitiveComponent Object Reference") (NormalImpulse :type "Object.Vector Structure") (Hit :type "EngineTypes.HitResult Structure (by ref)"))
  (bind _staticmesh (`self.StaticMesh`))
  (`GameplayStatics.PlaySoundAtLocation` "/Game/Sounds/item_created.item_created")
  (bind _output_get (set `self.hitpointshield1` (- (`self.hitpointshield1`) 1.0)))
  (if (<= _output_get 0.0)
    (`SceneComponent.SetHiddenInGame` _staticmesh true false)
    (`PrimitiveComponent.SetCollisionEnabled` _staticmesh "NoCollision")
    (`KismetSystemLibrary.K2_SetTimer` null "resetmesh1" 45.0)))

(event `self.StaticMesh1.OnComponentHit`
  (params (OtherActor :type "Actor Object Reference") (OtherComp :type "PrimitiveComponent Object Reference") (NormalImpulse :type "Object.Vector Structure") (Hit :type "EngineTypes.HitResult Structure (by ref)"))
  (bind _staticmesh1 (`self.StaticMesh1`))
  (`GameplayStatics.PlaySoundAtLocation` "/Game/Sounds/item_created.item_created")
  (bind _output_get (set `self.hitpointshield2` (- (`self.hitpointshield2`) 1.0)))
  (if (<= _output_get 0.0)
    (`SceneComponent.SetHiddenInGame` _staticmesh1 true false)
    (`PrimitiveComponent.SetCollisionEnabled` _staticmesh1 "NoCollision")
    (`KismetSystemLibrary.K2_SetTimer` null "resetmesh2" 45.0)))

(event `self.ReceiveActorBeginOverlap`
  (params (OtherActor :type "Actor Object Reference")))

(event `self.StaticMesh2.OnComponentHit`
  (params (OtherActor :type "Actor Object Reference") (OtherComp :type "PrimitiveComponent Object Reference") (NormalImpulse :type "Object.Vector Structure") (Hit :type "EngineTypes.HitResult Structure (by ref)"))
  (bind _staticmesh2 (`self.StaticMesh2`))
  (`GameplayStatics.PlaySoundAtLocation` "/Game/Sounds/item_created.item_created")
  (bind _output_get (set `self.hitpointshield3` (- (`self.hitpointshield3`) 1.0)))
  (if (<= _output_get 0.0)
    (`SceneComponent.SetHiddenInGame` _staticmesh2 true false)
    (`PrimitiveComponent.SetCollisionEnabled` _staticmesh2 "NoCollision")
    (`KismetSystemLibrary.K2_SetTimer` null "resetmesh3" 45.0)))

(event `self.StaticMesh3.OnComponentHit`
  (params (OtherActor :type "Actor Object Reference") (OtherComp :type "PrimitiveComponent Object Reference") (NormalImpulse :type "Object.Vector Structure") (Hit :type "EngineTypes.HitResult Structure (by ref)"))
  (bind _staticmesh3 (`self.StaticMesh3`))
  (`GameplayStatics.PlaySoundAtLocation` "/Game/Sounds/item_created.item_created" NormalImpulse)
  (bind _output_get (set `self.hitpointshield4` (- (`self.hitpointshield4`) 1.0)))
  (if (<= _output_get 0.0)
    (`SceneComponent.SetHiddenInGame` _staticmesh3 true false)
    (`PrimitiveComponent.SetCollisionEnabled` _staticmesh3 "NoCollision")
    (`KismetSystemLibrary.K2_SetTimer` null "resetmesh4" 45.0)))

(event `resetmesh1`
  (bind _staticmesh (`self.StaticMesh`))
  (set `self.hitpointshield1` 3.0)
  (`SceneComponent.SetHiddenInGame` _staticmesh false false)
  (`PrimitiveComponent.SetCollisionEnabled` _staticmesh "QueryAndPhysics"))

(event `resetmesh2`
  (bind _staticmesh1 (`self.StaticMesh1`))
  (set `self.hitpointshield2` 3.0)
  (`SceneComponent.SetHiddenInGame` _staticmesh1 false false)
  (`PrimitiveComponent.SetCollisionEnabled` _staticmesh1 "QueryAndPhysics"))

(event `resetmesh3`
  (bind _staticmesh2 (`self.StaticMesh2`))
  (set `self.hitpointshield3` 3.0)
  (`SceneComponent.SetHiddenInGame` _staticmesh2 false false)
  (`PrimitiveComponent.SetCollisionEnabled` _staticmesh2 "QueryAndPhysics"))

(event `resetmesh4`
  (bind _staticmesh3 (`self.StaticMesh3`))
  (set `self.hitpointshield4` 3.0)
  (`SceneComponent.SetHiddenInGame` _staticmesh3 false false)
  (`PrimitiveComponent.SetCollisionEnabled` _staticmesh3 "QueryAndPhysics"))

(fn `UserConstructionScript`)