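; Work-in-progress boss attack that spawns waves of Bomb actors from the AI_Boss1 found at BeginPlay.
; A looping timer, its interval randomised once at start, calls InitBombs to pick a Close, Mid, Far or Frontal wave.
; Close, Mid and Far waves can chain after short delays on coin flips, with Start flags tracking the entry wave to route the sequence.
; The Frontal wave is a standalone, larger burst.
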(event `self.ReceiveTick`
  (params (DeltaSeconds :type "Float (single-precision)")))

(event `self.ReceiveAnyDamage`
  (params (Damage :type "Float (single-precision)") (DamageType :type "DamageType Object Reference") (InstigatedBy :type "Controller Object Reference") (DamageCauser :type "Actor Object Reference")))

(event `self.ReceiveBeginPlay`
  (bind _outactors (`GameplayStatics.GetAllActorsOfClass` "/Game/Blueprints/ai/AI_Boss1.AI_Boss1_C"))
  (bind _asai_boss_1 (cast `/Game/Blueprints/ai/AI_Boss1` (`KismetArrayLibrary.Array_Get` _outactors)))
  (set `self.BossRef` _asai_boss_1)
  (`KismetSystemLibrary.K2_SetTimer` null "InitBombs" (`KismetMathLibrary.RandomFloatInRange` 4.0 12.0) true))

(event `InitBombs`
  (bind _bossref (`self.BossRef`))
  (bind _bossref_2 (`self.BossRef`))
  (bind _bossref_3 (`self.BossRef`))
  (bind _bossref_4 (`self.BossRef`))
  (switch `int` (`KismetMathLibrary.RandomIntegerInRange` 0 3)
    (:`Default`
      ;[1 1 1] Close Bomb Wave
      (`|SpawnActorFromClass` "/Game/Blueprints/Bomb.Bomb_C" (`SceneComponent.K2_GetComponentToWorld` _bossref_2) true :!label _label)
      (`|SpawnActorFromClass` "/Game/Blueprints/Bomb.Bomb_C" (`SceneComponent.K2_GetComponentToWorld` _bossref_2) true)
      (`|SpawnActorFromClass` "/Game/Blueprints/Bomb.Bomb_C" (`SceneComponent.K2_GetComponentToWorld` _bossref_2) true)
      (`|SpawnActorFromClass` "/Game/Blueprints/Bomb.Bomb_C" (`SceneComponent.K2_GetComponentToWorld` _bossref_2) true)
      (`|SpawnActorFromClass` "/Game/Blueprints/Bomb.Bomb_C" (`SceneComponent.K2_GetComponentToWorld` _bossref_2) true)
      (`|SpawnActorFromClass` "/Game/Blueprints/Bomb.Bomb_C" (`SceneComponent.K2_GetComponentToWorld` _bossref_2) true)
      (`|SpawnActorFromClass` "/Game/Blueprints/Bomb.Bomb_C" (`SceneComponent.K2_GetComponentToWorld` _bossref_2) true)
      (`|SpawnActorFromClass` "/Game/Blueprints/Bomb.Bomb_C" (`SceneComponent.K2_GetComponentToWorld` _bossref_2) true)
      (`KismetSystemLibrary.Delay` 0.5)
      (if (`self.startclose`)
        (if (== (`KismetMathLibrary.RandomIntegerInRange` 0 1) 0) :!label _label_2
          ;[1 1 1] Mid Bomb Wave
          (`|SpawnActorFromClass` "/Game/Blueprints/Bomb.Bomb_C" (`SceneComponent.K2_GetComponentToWorld` _bossref_3) true :!label _label_3)
          (`|SpawnActorFromClass` "/Game/Blueprints/Bomb.Bomb_C" (`SceneComponent.K2_GetComponentToWorld` _bossref_3) true)
          (`|SpawnActorFromClass` "/Game/Blueprints/Bomb.Bomb_C" (`SceneComponent.K2_GetComponentToWorld` _bossref_3) true)
          (`|SpawnActorFromClass` "/Game/Blueprints/Bomb.Bomb_C" (`SceneComponent.K2_GetComponentToWorld` _bossref_3) true)
          (`|SpawnActorFromClass` "/Game/Blueprints/Bomb.Bomb_C" (`SceneComponent.K2_GetComponentToWorld` _bossref_3) true)
          (`|SpawnActorFromClass` "/Game/Blueprints/Bomb.Bomb_C" (`SceneComponent.K2_GetComponentToWorld` _bossref_3) true)
          (`|SpawnActorFromClass` "/Game/Blueprints/Bomb.Bomb_C" (`SceneComponent.K2_GetComponentToWorld` _bossref_3) true)
          (`|SpawnActorFromClass` "/Game/Blueprints/Bomb.Bomb_C" (`SceneComponent.K2_GetComponentToWorld` _bossref_3) true)
          (`KismetSystemLibrary.Delay` 0.5)
          (if (`self.startclose`)
            (if (== (`KismetMathLibrary.RandomIntegerInRange` 0 1) 0) :!label _label_4
              ;[1 1 1] Far Bomb Wave
              (`|SpawnActorFromClass` "/Game/Blueprints/Bomb.Bomb_C" (`SceneComponent.K2_GetComponentToWorld` _bossref_4) true :!label _label_5)
              (`|SpawnActorFromClass` "/Game/Blueprints/Bomb.Bomb_C" (`SceneComponent.K2_GetComponentToWorld` _bossref_4) true)
              (`|SpawnActorFromClass` "/Game/Blueprints/Bomb.Bomb_C" (`SceneComponent.K2_GetComponentToWorld` _bossref_4) true)
              (`|SpawnActorFromClass` "/Game/Blueprints/Bomb.Bomb_C" (`SceneComponent.K2_GetComponentToWorld` _bossref_4) true)
              (`|SpawnActorFromClass` "/Game/Blueprints/Bomb.Bomb_C" (`SceneComponent.K2_GetComponentToWorld` _bossref_4) true)
              (`|SpawnActorFromClass` "/Game/Blueprints/Bomb.Bomb_C" (`SceneComponent.K2_GetComponentToWorld` _bossref_4) true)
              (`|SpawnActorFromClass` "/Game/Blueprints/Bomb.Bomb_C" (`SceneComponent.K2_GetComponentToWorld` _bossref_4) true)
              (`|SpawnActorFromClass` "/Game/Blueprints/Bomb.Bomb_C" (`SceneComponent.K2_GetComponentToWorld` _bossref_4) true)
              (`KismetSystemLibrary.Delay` 0.5)
              (if (`self.startclose`)
                _
                (elif (`self.startmid`)
                  (if (== (`KismetMathLibrary.RandomIntegerInRange` 0 1) 0) :!label _label_6
                    (goto _label)
                    (else
                      (set `self.startclose` false)
                      (set `self.startmid` false)
                      (set `self.startfar` false)))
                  (elif (`self.startfar`)
                    (goto _label_2))))
              (else
                (set `self.startclose` false)
                (set `self.startmid` false)
                (set `self.startfar` false)))
            (elif (`self.startmid`)
              (goto _label_4)
              (elif (`self.startfar`)
                (goto _label_6))))
          (else
            (set `self.startclose` false)
            (set `self.startmid` false)
            (set `self.startfar` false)))
        (elif (`self.startmid`)
          _
          (elif (`self.startfar`)
            _))))
    (:`0`
      (set `self.startclose` true)
      (goto _label))
    (:`1`
      (set `self.startmid` true)
      (goto _label_3))
    (:`2`
      (set `self.startfar` true)
      (goto _label_5))
    (:`3`
      ;[1 1 1] Frontal Bomb Wave
      (`|SpawnActorFromClass` "/Game/Blueprints/Bomb.Bomb_C" (`SceneComponent.K2_GetComponentToWorld` _bossref) true)
      (`|SpawnActorFromClass` "/Game/Blueprints/Bomb.Bomb_C" (`SceneComponent.K2_GetComponentToWorld` _bossref) true)
      (`|SpawnActorFromClass` "/Game/Blueprints/Bomb.Bomb_C" (`SceneComponent.K2_GetComponentToWorld` _bossref) true)
      (`|SpawnActorFromClass` "/Game/Blueprints/Bomb.Bomb_C" (`SceneComponent.K2_GetComponentToWorld` _bossref) true)
      (`|SpawnActorFromClass` "/Game/Blueprints/Bomb.Bomb_C" (`SceneComponent.K2_GetComponentToWorld` _bossref) true)
      (`|SpawnActorFromClass` "/Game/Blueprints/Bomb.Bomb_C" (`SceneComponent.K2_GetComponentToWorld` _bossref) true)
      (`|SpawnActorFromClass` "/Game/Blueprints/Bomb.Bomb_C" (`SceneComponent.K2_GetComponentToWorld` _bossref) true)
      (`|SpawnActorFromClass` "/Game/Blueprints/Bomb.Bomb_C" (`SceneComponent.K2_GetComponentToWorld` _bossref) true)
      (`|SpawnActorFromClass` "/Game/Blueprints/Bomb.Bomb_C" (`SceneComponent.K2_GetComponentToWorld` _bossref) true)
      (`|SpawnActorFromClass` "/Game/Blueprints/Bomb.Bomb_C" (`SceneComponent.K2_GetComponentToWorld` _bossref) true)
      (`|SpawnActorFromClass` "/Game/Blueprints/Bomb.Bomb_C" (`SceneComponent.K2_GetComponentToWorld` _bossref) true)
      (`|SpawnActorFromClass` "/Game/Blueprints/Bomb.Bomb_C" (`SceneComponent.K2_GetComponentToWorld` _bossref) true))))

(event `self.ReceiveActorBeginOverlap`
  (params (OtherActor :type "Actor Object Reference")))

(fn `UserConstructionScript`)