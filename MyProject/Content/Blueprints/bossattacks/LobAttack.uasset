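; LobAttack is a boss attack projectile that explodes on impact, dealing radial damage.
; On BeginPlay it caches the first AI_Boss1 in the level as the damage causer and instigator, and excludes it from the blast.
; HomingMissle2 turns on strong ProjectileMovement homing toward a supplied target component.
; On Hit it applies full, non-falloff radial damage, spawns an explosion emitter and destroys itself.
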(event `self.ReceiveActorBeginOverlap`
  (params (OtherActor :type "Actor Object Reference")))

(event `self.ReceiveBeginPlay`
  ;[1 1 1] Init
  (cast `/Game/Blueprints/MyCharacter` (`GameplayStatics.GetPlayerCharacter` 0))
  (bind _outactors (`GameplayStatics.GetAllActorsOfClass` "/Game/Blueprints/ai/AI_Boss1.AI_Boss1_C"))
  (bind _asai_boss_1 (cast `/Game/Blueprints/ai/AI_Boss1` (`KismetArrayLibrary.Array_Get` _outactors)))
  (set `self.BossRef` _asai_boss_1))

(event `Homing Missle2`
  (params (TargetToHit :type "PrimitiveComponent Object Reference"))
  (bind _projectilemovement (`self.ProjectileMovement`))
  ;[1 1 1] Home
  (if (`KismetSystemLibrary.IsValid` TargetToHit)
    (set `ProjectileMovementComponent.HomingTargetComponent` TargetToHit _projectilemovement)
    (set `ProjectileMovementComponent.bIsHomingProjectile` true _projectilemovement)
    (set `ProjectileMovementComponent.HomingAccelerationMagnitude` 40000.0 _projectilemovement)))

(event `self.ReceiveHit`
  (params (MyComp :type "PrimitiveComponent Object Reference") (Other :type "Actor Object Reference") (OtherComp :type "PrimitiveComponent Object Reference") (bSelfMoved :type Boolean) (HitLocation :type "Object.Vector Structure") (HitNormal :type "Object.Vector Structure") (NormalImpulse :type "Object.Vector Structure") (Hit :type "EngineTypes.HitResult Structure (by ref)"))
  (bind _bossref (`self.BossRef`))
  ;[1 1 1] Hit
  (`GameplayStatics.ApplyRadialDamage` (`self.damage`) (`self.K2_GetActorLocation`) 250.0 null (`|MakeArray` _bossref :!type "Actor Object Reference") _bossref (`Pawn.GetController` _bossref) true)
  (`GameplayStatics.SpawnEmitterAtLocation` "/Game/StarterContent/Particles/P_Explosion.P_Explosion" HitLocation)
  (`self.K2_DestroyActor`))

(fn `UserConstructionScript`)