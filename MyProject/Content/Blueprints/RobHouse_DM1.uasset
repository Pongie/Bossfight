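; RobHouse_DM1 is a destructible house that varies its look and size in the construction script.
; The script picks random wall and roof materials for its slots, applies a randomized actor scale and enables collision.
; When the destructible fractures, it passes the Sphere's location to RandomOrb's break handler, disables collision and destroys the actor after a short delay.
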(event `self.ReceiveBeginPlay`)

(event `self.ReceiveActorBeginOverlap`
  (params (OtherActor :type "Actor Object Reference")))

(event `self.ReceiveTick`
  (params (DeltaSeconds :type "Float (single-precision)")))

(event `self.Destructible.OnComponentFracture`
  (params (HitPoint :type "Object.Vector Structure (by ref)") (HitDirection :type "Object.Vector Structure (by ref)"))
  (`/Game/Blueprints/RandomOrb.Ondestructbreak` (`self.RandomOrb`) (`KismetMathLibrary.MakeTransform` (`SceneComponent.K2_GetComponentLocation` (`self.Sphere`)) (struct) (1.0 1.0 1.0)))
  (`PrimitiveComponent.SetCollisionEnabled` "NoCollision")
  (`KismetSystemLibrary.Delay` 2.5)
  (`self.K2_DestroyActor`))

(fn `UserConstructionScript`
  (bind _item (`KismetArrayLibrary.Array_Get` (`self.Roof Materials`) (`KismetMathLibrary.RandomIntegerInRange` 0 2)))
  (`PrimitiveComponent.SetMaterial` 1 (`KismetArrayLibrary.Array_Get` (`self.Wall Materials`) (`KismetMathLibrary.RandomIntegerInRange` 0 1)))
  (`PrimitiveComponent.SetMaterial` 2 _item)
  (`PrimitiveComponent.SetMaterial` 4 _item)
  (`self.SetActorScale3D` (+ (`KismetMathLibrary.MakeVector` (* (`KismetMathLibrary.RandomFloat`) 2.0) (* (`KismetMathLibrary.RandomFloat`) 2.0) (* (`KismetMathLibrary.RandomFloat`) 3.0)) (15.0 15.0 15.0)))
  (`PrimitiveComponent.SetCollisionEnabled` "QueryAndPhysics"))