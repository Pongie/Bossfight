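; Blueprint that spawns a random elemental orb, apparently when a destructible object breaks.
; Ondestructbreak calls Randomorb to roll an integer, then branches on it to spawn a Fire, Water or Wind actor at the passed-in transform, ignoring collisions.
; Each branch prints the element name for debugging; the event graph is empty and some debug prints are left disconnected.
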(event `self.ReceiveTick`
  (params (DeltaSeconds :type "Float (single-precision)")))

(event `self.ReceiveInitializeComponent`)

(fn `Ondestructbreak`
  (params (sheet :type "Object.Transform Structure"))
  (bind _currentorb (`self.CurrentOrb`))
  (`self.randomorb`)
  (if (== (`self.CurrentOrb`) 0)
    (`|SpawnActorFromClass` "/Game/Blueprints/Items/Fire.Fire_C" sheet true)
    (`KismetSystemLibrary.PrintString` "Fire")
    (elif (== (`self.CurrentOrb`) 1)
      (`|SpawnActorFromClass` "/Game/Blueprints/Items/Water.Water_C" sheet true)
      (`KismetSystemLibrary.PrintString` "Water")
      (elif (== _currentorb 2)
        (`|SpawnActorFromClass` "/Game/Blueprints/Items/Wind.Wind_C" sheet true)
        (`KismetSystemLibrary.PrintString` "Wind")
        (else
          (`KismetSystemLibrary.PrintString` (`KismetStringLibrary.Conv_IntToString` _currentorb)))))))

(fn `randomorb`
  (set `self.Currentorb` (`KismetMathLibrary.RandomIntegerInRange` 0 2)))