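; Ragdoll stand-in actor that takes on the skeletal mesh of the boss present in the level.
; On BeginPlay it casts the first AI_Boss1 found to Guardian, Scarab or NewPlot and sets Bossvar to match.
; A switch applies the mesh, greatly upscaling Guardian and Scarab, then enables physics and collision, ignoring GameTraceChannel1.
; A Skeleton mesh case exists, but no cast selects it.
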(event `self.ReceiveBeginPlay`
  (bind _mesh (`self.Mesh`))
  (bind _outactors (`GameplayStatics.GetAllActorsOfClass` "/Game/Blueprints/ai/AI_Boss1.AI_Boss1_C"))
  (bind _item (`KismetArrayLibrary.Array_Get` _outactors))
  (cast `/Game/Blueprints/ai/AI_Boss_Guardian` _item
    (:`then`
      (set `self.bossvar` 1))
    (:`CastFailed`
      (cast `/Game/Blueprints/ai/AI_Boss1_Scarab` _item
        (:`then`
          (set `self.bossvar` 2))
        (:`CastFailed`
          (cast `/Game/Blueprints/ai/AI_Boss1_NewPlot` _item)
          (set `self.bossvar` 0)))))
  (switch `int` (`self.bossvar`)
    (:`Default`
      (`SkinnedMeshComponent.SetSkinnedAssetAndUpdate` _mesh (`self.PlotBoss`) :!label _label))
    (:`0`
      (goto _label))
    (:`1`
      (`SkinnedMeshComponent.SetSkinnedAssetAndUpdate` _mesh (`self.GuardianBoss`))
      (`self.SetActorScale3D` (299.0 299.0 299.0)))
    (:`2`
      (`SkinnedMeshComponent.SetSkinnedAssetAndUpdate` _mesh (`self.ScarabBoss`))
      (`self.SetActorScale3D` (299.0 299.0 299.0)))
    (:`3`
      (`SkinnedMeshComponent.SetSkinnedAssetAndUpdate` _mesh (`self.SkeletonBoss`))))
  (`PrimitiveComponent.SetSimulatePhysics` true)
  (`PrimitiveComponent.SetCollisionEnabled` "QueryAndPhysics")
  (`PrimitiveComponent.SetCollisionResponseToChannel` "ECC_GameTraceChannel1" "ECR_Ignore")
  (`PrimitiveComponent.SetCollisionResponseToChannel` "ECC_GameTraceChannel1" "ECR_Ignore"))

(event `self.ReceiveActorBeginOverlap`
  (params (OtherActor :type "Actor Object Reference")))

(event `self.ReceiveTick`
  (params (DeltaSeconds :type "Float (single-precision)")))

(fn `UserConstructionScript`)