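; Character select screen controller for one player slot, handling join, ready-up and appearance choices on placed preview actors.
; Jump first joins, revealing the preview and raising the game instance's PlayerCount; later presses set ready and increment ReadyPlayers, with no repeat guard.
; Once joined, attack inputs toggle gender, cycle four weapons and cycle four material colors on both bodies.
; Weapon and color choices are written to MyGameInstance arrays by PlayerNum; gender is not saved.
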(event `InputAction|Jump`
  ;[1 1 1] Join-In
  (:`Pressed`
    (if (`self.joined`)
      (set `self.isReady` true)
      (bind _readyplayers (`/Game/Blueprints/MyGameInstance.readyPlayers` (stale _asmy_game_instance)))
      (set `/Game/Blueprints/MyGameInstance.readyPlayers` (+ _readyplayers 1) (stale _asmy_game_instance))
      (`KismetSystemLibrary.PrintString` (`KismetStringLibrary.Conv_IntToString` _readyplayers))
      (else
        (`self.SetActorHiddenInGame` (`self.Male`) false)
        (`self.SetActorHiddenInGame` (`self.Bow`) false)
        (set `self.joined` true)
        (bind _asmy_game_instance (cast `/Game/Blueprints/MyGameInstance` (`GameplayStatics.GetGameInstance`))
          (:`then`
            (set `/Game/Blueprints/MyGameInstance.playerCount` (+ (`/Game/Blueprints/MyGameInstance.playerCount` _asmy_game_instance) 1) _asmy_game_instance))
          (:`CastFailed`
            (`KismetSystemLibrary.PrintString` "should increment count")))))))

(event `InputAction|Attack Action 1`
  ;[1 1 1] Gender Swap
  (:`Pressed`
    (if (`self.joined`)
      (if (`self.isMale`)
        (`self.SetActorHiddenInGame` (`self.Male`) true)
        (`self.SetActorHiddenInGame` (`self.Female`) false)
        (set `self.isMale` false)
        (else
          (`self.SetActorHiddenInGame` (`self.Male`) false)
          (`self.SetActorHiddenInGame` (`self.Female`) true)
          (set `self.isMale` true))))))

(event `self.ReceiveActorBeginOverlap`
  (params (OtherActor :type "Actor Object Reference")))

(event `self.ReceiveTick`
  (params (DeltaSeconds :type "Float (single-precision)")))

(event `InputAction|Attack Action 2`
  ;[1 1 1] Weapon Swap
  (:`Pressed`
    (if (`self.joined`)
      (switch `int` (`self.weaponNumber`)
        (:`0`
          (`self.SetActorHiddenInGame` (`self.Bow`) true)
          (`self.SetActorHiddenInGame` (`self.Spear`) false)
          (set `self.weaponNumber` 1))
        (:`1`
          (`self.SetActorHiddenInGame` (`self.Spear`) true)
          (`self.SetActorHiddenInGame` (`self.Sword`) false)
          (set `self.weaponNumber` 2))
        (:`2`
          (`self.SetActorHiddenInGame` (`self.Sword`) true)
          (`self.SetActorHiddenInGame` (`self.Staff`) false)
          (set `self.weaponNumber` 3))
        (:`3`
          (`self.SetActorHiddenInGame` (`self.Staff`) true)
          (`self.SetActorHiddenInGame` (`self.Bow`) false)
          (set `self.weaponNumber` 0)))
      (bind _asmy_game_instance (cast `/Game/Blueprints/MyGameInstance` (`GameplayStatics.GetGameInstance`)))
      (`KismetArrayLibrary.Array_Set` (`/Game/Blueprints/MyGameInstance.playerWeaponChoices` _asmy_game_instance) (`self.playerNum`) (`self.weaponNumber`)))))

(event `InputAction|Attack Action 3`
  ;[1 1 1] Color Swap
  (:`Pressed`
    (if (`self.joined`)
      (switch `int` (`self.colorNumber`)
        (:`0`
          (`|ExecutionSequence`
            (:`then_0`
              (bind _asskeletal_mesh_actor (cast `SkeletalMeshActor` (`self.Male`)))
              (`PrimitiveComponent.SetMaterial` (`SkeletalMeshActor.SkeletalMeshComponent` _asskeletal_mesh_actor) 0 null))
            (:`then_1`
              (bind _asskeletal_mesh_actor_2 (cast `SkeletalMeshActor` (`self.Female`)))
              (`PrimitiveComponent.SetMaterial` (`SkeletalMeshActor.SkeletalMeshComponent` _asskeletal_mesh_actor_2) 0 null)))
          (set `self.colorNumber` 1))
        (:`1`
          (`|ExecutionSequence`
            (:`then_0`
              (bind _asskeletal_mesh_actor_3 (cast `SkeletalMeshActor` (`self.Male`)))
              (`PrimitiveComponent.SetMaterial` (`SkeletalMeshActor.SkeletalMeshComponent` _asskeletal_mesh_actor_3) 0 null))
            (:`then_1`
              (bind _asskeletal_mesh_actor_4 (cast `SkeletalMeshActor` (`self.Female`)))
              (`PrimitiveComponent.SetMaterial` (`SkeletalMeshActor.SkeletalMeshComponent` _asskeletal_mesh_actor_4) 0 null)))
          (set `self.colorNumber` 2))
        (:`2`
          (`|ExecutionSequence`
            (:`then_0`
              (bind _asskeletal_mesh_actor_5 (cast `SkeletalMeshActor` (`self.Male`)))
              (`PrimitiveComponent.SetMaterial` (`SkeletalMeshActor.SkeletalMeshComponent` _asskeletal_mesh_actor_5) 0 null))
            (:`then_1`
              (bind _asskeletal_mesh_actor_6 (cast `SkeletalMeshActor` (`self.Female`)))
              (`PrimitiveComponent.SetMaterial` (`SkeletalMeshActor.SkeletalMeshComponent` _asskeletal_mesh_actor_6) 0 null)))
          (set `self.colorNumber` 3))
        (:`3`
          (`|ExecutionSequence`
            (:`then_0`
              (bind _asskeletal_mesh_actor_7 (cast `SkeletalMeshActor` (`self.Male`)))
              (`PrimitiveComponent.SetMaterial` (`SkeletalMeshActor.SkeletalMeshComponent` _asskeletal_mesh_actor_7) 0 null))
            (:`then_1`
              (bind _asskeletal_mesh_actor_8 (cast `SkeletalMeshActor` (`self.Female`)))
              (`PrimitiveComponent.SetMaterial` (`SkeletalMeshActor.SkeletalMeshComponent` _asskeletal_mesh_actor_8) 0 null)))
          (set `self.colorNumber` 0)))
      (bind _asmy_game_instance (cast `/Game/Blueprints/MyGameInstance` (`GameplayStatics.GetGameInstance`)))
      (`KismetArrayLibrary.Array_Set` (`/Game/Blueprints/MyGameInstance.playerColorChoices` _asmy_game_instance) (`self.playerNum`) (`self.colorNumber`)))))

(fn `UserConstructionScript`)