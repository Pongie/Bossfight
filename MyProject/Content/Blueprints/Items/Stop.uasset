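; Stop is an item Blueprint whose Use function is meant to act on the AI_Boss1 boss.
; Use clears the boss's IsStunned flag if set and returns false, but the cast to AI_Boss1 has no object wired in and the Player argument is unused.
; Disconnected nodes that would spawn a scaled-down Stop and set Thrown never run, and the event graph holds only placeholders.
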(event `self.ReceiveBeginPlay`)

(event `self.ReceiveActorBeginOverlap`
  (params (OtherActor :type "Actor Object Reference"))
  (`parent.ReceiveActorBeginOverlap` null))

(event `self.ReceiveTick`
  (params (DeltaSeconds :type "Float (single-precision)")))

(fn `Use`
  (params (Player :type "/Game/Blueprints/MyCharacter Object Reference"))
  (returns (NewParam :type Boolean))
  (bind _asai_boss_1 (cast `/Game/Blueprints/ai/AI_Boss1` null))
  (if (`/Game/Blueprints/ai/AI_Boss1.isStunned` _asai_boss_1)
    (set `/Game/Blueprints/ai/AI_Boss1.isStunned` false _asai_boss_1)
    (return false)))

(fn `UserConstructionScript`
  (`parent.UserConstructionScript`))