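; Explosive item that, when used, spawns an enlarged copy of itself marked as Thrown, offset from the player along world X rather than player facing.
; The copy ignores a custom collision channel, and Use returns false.
; On hit, a thrown copy deals full radial damage, sparing MyCharacter actors cached at BeginPlay.
; It then spawns an explosion effect, plays a sound at world origin and destroys itself.
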(event `self.ReceiveHit`
  (params (MyComp :type "PrimitiveComponent Object Reference") (Other :type "Actor Object Reference") (OtherComp :type "PrimitiveComponent Object Reference") (bSelfMoved :type Boolean) (HitLocation :type "Object.Vector Structure") (HitNormal :type "Object.Vector Structure") (NormalImpulse :type "Object.Vector Structure") (Hit :type "EngineTypes.HitResult Structure (by ref)"))
  (if (`self.thrown`)
    (`GameplayStatics.ApplyRadialDamage` 50.0 HitLocation 500.0 null (stale `self.ReceiveBeginPlay` _outactors) self null true)
    (`GameplayStatics.SpawnEmitterAtLocation` "/Game/StarterContent/Particles/P_Explosion.P_Explosion" HitLocation)
    (`GameplayStatics.PlaySoundAtLocation` "/Game/StarterContent/Audio/Explosion02.Explosion02")
    (`self.K2_DestroyActor`)))

(event `self.ReceiveActorBeginOverlap`
  (params (OtherActor :type "Actor Object Reference"))
  (`parent.ReceiveActorBeginOverlap` null))

(event `self.ReceiveBeginPlay`
  (bind _outactors (`GameplayStatics.GetAllActorsOfClass` "/Game/Blueprints/MyCharacter.MyCharacter_C")))

(event `self.ReceiveTick`
  (params (DeltaSeconds :type "Float (single-precision)")))

(fn `Use`
  (params (Player :type "/Game/Blueprints/MyCharacter Object Reference"))
  (returns (NewParam :type Boolean))
  (bind _returnvalue (`|SpawnActorFromClass` "Explosive_C" (`KismetMathLibrary.MakeTransform` (+ (`self.K2_GetActorLocation` Player) (* (`KismetMathLibrary.GetForwardVector` (struct)) 100.0)) (`self.K2_GetActorRotation` Player) (5.0 5.0 5.0)) true))
  (set `/Game/Blueprints/Items/Explosive.thrown` true _returnvalue)
  (`PrimitiveComponent.SetCollisionResponseToChannel` _returnvalue "ECC_GameTraceChannel1" "ECR_Ignore")
  (return false))

(fn `UserConstructionScript`
  (`parent.UserConstructionScript`))