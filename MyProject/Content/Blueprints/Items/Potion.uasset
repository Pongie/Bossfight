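; Potion is an item Blueprint that restores health to the player who uses it.
; Its Use function adds PotionPoints to the player's CurrentHealth if the player is not dead, with no clamp to a maximum in this function.
; Use returns false whether or not healing happens.
; The event graph holds only disabled default nodes, and the construction script just calls its parent.
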(event `self.ReceiveBeginPlay`)

(event `self.ReceiveActorBeginOverlap`
  (params (OtherActor :type "Actor Object Reference"))
  (`parent.ReceiveActorBeginOverlap` null))

(event `self.ReceiveTick`
  (params (DeltaSeconds :type "Float (single-precision)")))

(fn `Use`
  (params (Player :type "/Game/Blueprints/MyCharacter Object Reference"))
  (returns (NewParam :type Boolean))
  (if (not (`/Game/Blueprints/MyCharacter.isDead` Player))
    (set `/Game/Blueprints/MyCharacter.CurrentHealth` (+ (`/Game/Blueprints/MyCharacter.CurrentHealth` Player) (`self.potionPoints`)) Player))
  (return false))

(fn `UserConstructionScript`
  (`parent.UserConstructionScript`))