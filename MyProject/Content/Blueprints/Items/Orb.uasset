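; Orb item that buffs two chosen stats (max health, speed or strength) on a MyCharacter and can remove the buff.
; OrbifyPlayer switches on Stat1 and Stat2 to add modifiers, though Stat1's speed and strength cases use StatMod2.
; DeorbifyPlayer subtracts health modifiers but sets speed and strength to zero, leaving its subtraction nodes unused.
; The event graph is empty, so nothing here calls either function.
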(event `self.ReceiveBeginPlay`)

(event `self.ReceiveActorBeginOverlap`
  (params (OtherActor :type "Actor Object Reference")))

(event `self.ReceiveTick`
  (params (DeltaSeconds :type "Float (single-precision)")))

(fn `de-orbifyPlayer`
  (params (targetPlayer :type "/Game/Blueprints/MyCharacter Object Reference"))
  (returns (NewParam :type Boolean))
  ;[1 1 1] If the tooltips are to be believed, the INT setters should work normally arranged as they are.
  (bind _asmy_character (cast `/Game/Blueprints/MyCharacter` targetPlayer))
  (switch `string` (`self.stat1`)
    (:`Health`
      (set `/Game/Blueprints/MyCharacter.Maxhealth` (- (`/Game/Blueprints/MyCharacter.Maxhealth` _asmy_character) (`KismetMathLibrary.Conv_IntToDouble` (`self.statMod1`))) _asmy_character))
    (:`Speed`
      (bind _output_get (set `/Game/Blueprints/MyCharacter.playerSpeed` 0 _asmy_character)))
    (:`Strength`
      (bind _output_get_2 (set `/Game/Blueprints/MyCharacter.playerStrength` 0 _asmy_character))))
  (switch `string` (`self.stat2`)
    (:`Default`
      _)
    (:`Health`
      (set `/Game/Blueprints/MyCharacter.Maxhealth` (- (`/Game/Blueprints/MyCharacter.Maxhealth` _asmy_character) (`KismetMathLibrary.Conv_IntToDouble` (`self.statMod2`))) _asmy_character))
    (:`Speed`
      (bind _output_get_3 (set `/Game/Blueprints/MyCharacter.playerSpeed` 0 _asmy_character)))
    (:`Strength`
      (bind _output_get_4 (set `/Game/Blueprints/MyCharacter.playerStrength` 0 _asmy_character))))
  (return false))

(fn `orbifyPlayer`
  (params (targetPlayer :type "/Game/Blueprints/MyCharacter Object Reference"))
  (returns (NewParam :type Boolean))
  ;[1 1 1] If the tooltips are to be believed, the INT setters should work normally arranged as they are.
  (bind _asmy_character (cast `/Game/Blueprints/MyCharacter` targetPlayer)
    (:`then`
      (switch `string` (`self.stat1`)
        (:`Health`
          (set `/Game/Blueprints/MyCharacter.Maxhealth` (+ (`/Game/Blueprints/MyCharacter.Maxhealth` _asmy_character) (`KismetMathLibrary.Conv_IntToDouble` (`self.statMod1`))) _asmy_character))
        (:`Speed`
          (set `/Game/Blueprints/MyCharacter.playerSpeed` (+ (`/Game/Blueprints/MyCharacter.playerSpeed` _asmy_character) (`self.statMod2`)) _asmy_character))
        (:`Strength`
          (set `/Game/Blueprints/MyCharacter.playerStrength` (+ (`/Game/Blueprints/MyCharacter.playerStrength` _asmy_character) (`self.statMod2`)) _asmy_character)))
      (switch `string` (`self.stat2`)
        (:`Health`
          (set `/Game/Blueprints/MyCharacter.Maxhealth` (+ (`/Game/Blueprints/MyCharacter.Maxhealth` _asmy_character) (`KismetMathLibrary.Conv_IntToDouble` (`self.statMod2`))) _asmy_character))
        (:`Speed`
          (set `/Game/Blueprints/MyCharacter.playerSpeed` (+ (`/Game/Blueprints/MyCharacter.playerSpeed` _asmy_character) (`self.statMod2`)) _asmy_character))
        (:`Strength`
          (set `/Game/Blueprints/MyCharacter.playerStrength` (+ (`/Game/Blueprints/MyCharacter.playerStrength` _asmy_character) (`self.statMod2`)) _asmy_character)))
      (return true))
    (:`CastFailed`
      (`KismetSystemLibrary.PrintString` "Orbify cast failed"))))

(fn `UserConstructionScript`
  (`parent.UserConstructionScript`))