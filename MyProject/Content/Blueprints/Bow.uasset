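; Bow weapon that gives the player three arrow attacks, each gated by a game-time cooldown and scaled by PlayerStrength.
; Attack1 fires a single arrow, while Attack2 fires a three-arrow fan with raised gravity to shorten range.
; Attack3 calls a dispatcher into an EventGraph Delay loop that charges while Holdbutton is held.
; Release or maximum charge fires a Charged_Projectile whose speed, size and extra damage grow with charge.
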(event `self.ReceiveTick`
  (params (DeltaSeconds :type "Float (single-precision)")))

(event `self.ReceiveActorBeginOverlap`
  (params (OtherActor :type "Actor Object Reference")))

(event `self.ReceiveBeginPlay`
  (add `self.Attack3Event` (delegate `Attack3Event_Event`)))

(event `Attack3Event_Event`
  (bind _myplayer (`self.myPlayer`))
  (bind _arrowmaxspeed (`self.Arrowmaxspeed`))
  (bind _arrowsizeincrease (`self.Arrowsizeincrease`))
  (bind _returnvalue (`self.K2_GetActorRotation` _myplayer))
  (`/Engine/EditorBlueprintResources/StandardMacros.CompareFloat` (`self.CoolDown3`) (`KismetSystemLibrary.GetGameTimeInSeconds`)
    (:`<`
      (if (`/Game/Blueprints/MyCharacter.holdbutton` (`self.myPlayer`)) :!label _label
        (if (< _arrowmaxspeed 5000.0)
          (set `self.Arrowmaxspeed` (+ _arrowmaxspeed 400.0))
          (set `self.Arrowsizeincrease` (+ (`self.Arrowsizeincrease`) (0.08 0.08 0.08)))
          (`KismetSystemLibrary.Delay` 0.05)
          (goto _label)
          (else
            _)))
      (bind _returnvalue_2 (`|SpawnActorFromClass` "/Game/Blueprints/Charged_Projectile.Charged_Projectile_C" (`KismetMathLibrary.MakeTransform` (+ (`self.K2_GetActorLocation` _myplayer) (* (`KismetMathLibrary.GetForwardVector` _returnvalue) 200.0)) _returnvalue (0.3 0.3 0.3)) true (`/Game/Blueprints/MyCharacter.playerStrength` _myplayer)))
      (`self.SetLifeSpan` _returnvalue_2 2.0)
      (`self.SetActorScale3D` _returnvalue_2 _arrowsizeincrease)
      (bind _projectilemovement (`/Game/Blueprints/Charged_Projectile.ProjectileMovement` _returnvalue_2))
      (set `MovementComponent.Velocity` (* (`MovementComponent.Velocity` _projectilemovement) (`self.Arrowmaxspeed`)) _projectilemovement)
      (set `/Game/Blueprints/Charged_Projectile.extraDamage` (* (.z _arrowsizeincrease) 10.0) _returnvalue_2)
      (set `self.Arrowmaxspeed` 0.0)
      (set `self.Arrowsizeincrease` (0.0 0.0 0.0))
      (set `self.CoolDown3` (+ (`KismetSystemLibrary.GetGameTimeInSeconds`) 3.0)))))

(fn `Attack1`
  (returns (NewParam :type Boolean))
  (bind _myplayer (`self.myPlayer`))
  (bind _returnvalue (`self.K2_GetActorRotation` _myplayer))
  (`/Engine/EditorBlueprintResources/StandardMacros.CompareFloat` (`self.CoolDown1`) (`KismetSystemLibrary.GetGameTimeInSeconds`)
    (:`<`
      (bind _returnvalue_2 (`|SpawnActorFromClass` "/Game/Blueprints/Projectile.Projectile_C" (`KismetMathLibrary.MakeTransform` (+ (`self.K2_GetActorLocation` _myplayer) (* (`KismetMathLibrary.GetForwardVector` _returnvalue) 100.0)) _returnvalue (0.3 0.3 0.3)) false 1.0))
      (`self.SetLifeSpan` _returnvalue_2 (`self.Arrowlifespan`))
      (set `/Game/Blueprints/Projectile.Base_Damageprojectile` (`/Game/Blueprints/MyCharacter.playerStrength` _myplayer) _returnvalue_2)
      (set `self.CoolDown1` (+ (`KismetSystemLibrary.GetGameTimeInSeconds`) 0.5))
      (return false))))

(fn `Attack2`
  (returns (NewParam :type Boolean))
  (bind _myplayer (`self.myPlayer`))
  (bind _myplayer_2 (`self.myPlayer`))
  (bind _arrowlifespan (`self.Arrowlifespan`))
  (bind _returnvalue (`self.K2_GetActorRotation` _myplayer_2))
  (bind _returnvalue_2 (`self.K2_GetActorRotation` _myplayer))
  (bind _returnvalue_3 (`self.K2_GetActorRotation` _myplayer_2))
  (bind _playerstrength (`/Game/Blueprints/MyCharacter.playerStrength` _myplayer))
  (`/Engine/EditorBlueprintResources/StandardMacros.CompareFloat` (`self.CoolDown2`) (`KismetSystemLibrary.GetGameTimeInSeconds`)
    (:`<`
      (bind _returnvalue_4 (`|SpawnActorFromClass` "/Game/Blueprints/Projectile.Projectile_C" (`KismetMathLibrary.MakeTransform` (+ (`self.K2_GetActorLocation` _myplayer) (* (`KismetMathLibrary.GetForwardVector` _returnvalue_2) 100.0)) _returnvalue_2 (0.3 0.3 0.3)) false 1.0))
      (`self.SetLifeSpan` _returnvalue_4 _arrowlifespan)
      (set `/Game/Blueprints/Projectile.Base_Damageprojectile` _playerstrength _returnvalue_4)
      (bind _projectilemovement (`/Game/Blueprints/Projectile.ProjectileMovement` _returnvalue_4))
      (set `ProjectileMovementComponent.ProjectileGravityScale` (+ (`ProjectileMovementComponent.ProjectileGravityScale` _projectilemovement) 0.33) _projectilemovement)
      (bind _returnvalue_5 (`|SpawnActorFromClass` "/Game/Blueprints/Projectile.Projectile_C" (`KismetMathLibrary.MakeTransform` (+ (`self.K2_GetActorLocation` _myplayer) (* (`KismetMathLibrary.GetForwardVector` _returnvalue_3) 100.0)) (`KismetMathLibrary.MakeRot` (.pitch _returnvalue_3) (+ (.yaw _returnvalue_3) 20.0) (.roll _returnvalue_3)) (0.3 0.3 0.3)) false 1.0))
      (`self.SetLifeSpan` _returnvalue_5 _arrowlifespan)
      (set `/Game/Blueprints/Projectile.Base_Damageprojectile` _playerstrength _returnvalue_5)
      (bind _projectilemovement_2 (`/Game/Blueprints/Projectile.ProjectileMovement` _returnvalue_5))
      (set `ProjectileMovementComponent.ProjectileGravityScale` (+ (`ProjectileMovementComponent.ProjectileGravityScale` _projectilemovement_2) 0.33) _projectilemovement_2)
      (bind _returnvalue_6 (`|SpawnActorFromClass` "/Game/Blueprints/Projectile.Projectile_C" (`KismetMathLibrary.MakeTransform` (+ (`self.K2_GetActorLocation` _myplayer_2) (* (`KismetMathLibrary.GetForwardVector` _returnvalue) 100.0)) (`KismetMathLibrary.MakeRot` (.pitch _returnvalue) (- (.yaw _returnvalue) 20.0) (.roll _returnvalue)) (0.3 0.3 0.3)) false 1.0))
      (`self.SetLifeSpan` _returnvalue_6 _arrowlifespan)
      (set `/Game/Blueprints/Projectile.Base_Damageprojectile` _playerstrength _returnvalue_6)
      (bind _projectilemovement_3 (`/Game/Blueprints/Projectile.ProjectileMovement` _returnvalue_6))
      (set `ProjectileMovementComponent.ProjectileGravityScale` (+ (`ProjectileMovementComponent.ProjectileGravityScale` _projectilemovement_3) 0.33) _projectilemovement_3)
      (set `self.CoolDown2` (+ (`KismetSystemLibrary.GetGameTimeInSeconds`) 2.0))
      (return false))))

(fn `Attack3`
  (returns (NewParam :type Boolean))
  (`self.Attack3Event`)
  (return false))

(fn `UserConstructionScript`
  (`parent.UserConstructionScript`))