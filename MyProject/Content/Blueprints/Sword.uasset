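; Sword actor that serves as the player's melee weapon and damages actors it hits.
; On BeginPlay it shows or hides its mesh according to the player character's Swordequipped flag.
; Its Hit event applies MeleeDamage to the struck actor and plays an explosion sound at the impact point.
; Capsule hitbox spawning and timed visibility logic remain as disconnected, unused nodes in both graphs.
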(event `self.ReceiveBeginPlay`
  (bind _swordmesh (`self.swordmesh`))
  (bind _asmy_character (cast `/Game/Blueprints/MyCharacter` (`GameplayStatics.GetPlayerCharacter` 0))
    (:`then`
      (if (`/Game/Blueprints/MyCharacter.swordequipped` _asmy_character)
        (`SceneComponent.SetHiddenInGame` _swordmesh false false)
        (else
          (`SceneComponent.SetHiddenInGame` _swordmesh true false))))
    (:`CastFailed`
      (`KismetSystemLibrary.PrintString` "?"))))

(event `self.ReceiveHit`
  (params (MyComp :type "PrimitiveComponent Object Reference") (Other :type "Actor Object Reference") (OtherComp :type "PrimitiveComponent Object Reference") (bSelfMoved :type Boolean) (HitLocation :type "Object.Vector Structure") (HitNormal :type "Object.Vector Structure") (NormalImpulse :type "Object.Vector Structure") (Hit :type "EngineTypes.HitResult Structure (by ref)"))
  ;[1 1 1] Assign Projectile Vars (Based off Bow)
  (`KismetSystemLibrary.PrintString` "Hitting")
  (`GameplayStatics.ApplyDamage` Other (`self.MeleeDamage`) null self)
  (`GameplayStatics.PlaySoundAtLocation` "/Game/StarterContent/Audio/Explosion02.Explosion02" HitLocation))

(event `self.ReceiveActorBeginOverlap`
  (params (OtherActor :type "Actor Object Reference")))

(fn `UserConstructionScript`
  (`parent.UserConstructionScript`))