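; Revive Blueprint that brings the player character back from death through a TestRevive function.
; TestRevive casts player zero to MyCharacter and, if IsDead is set, restores a fixed amount of health and clears the flag.
; Debug strings print on every call and when the cast fails.
; The event graph holds only disabled placeholder events, so nothing in this asset calls the function itself.
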(event `self.ReceiveBeginPlay`)

(event `self.ReceiveActorBeginOverlap`
  (params (OtherActor :type "Actor Object Reference"))
  (`parent.ReceiveActorBeginOverlap` null))

(fn `TestRevive`
  (`KismetSystemLibrary.PrintString` "hey senpai")
  (bind _asmy_character (cast `/Game/Blueprints/MyCharacter` (`GameplayStatics.GetPlayerCharacter` 0))
    (:`then`
      (if (`/Game/Blueprints/MyCharacter.isDead` _asmy_character)
        (set `/Game/Blueprints/MyCharacter.CurrentHealth` 50.0 _asmy_character)
        (set `/Game/Blueprints/MyCharacter.isDead` false _asmy_character)))
    (:`CastFailed`
      (`KismetSystemLibrary.PrintString` "seMpai"))))

(fn `UserConstructionScript`
  (`parent.UserConstructionScript`))