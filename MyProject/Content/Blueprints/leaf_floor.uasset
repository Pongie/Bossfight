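; Leaf floor actor that temporarily disappears when a lob attack actor overlaps it.
; On overlap it casts its LobAttack reference and proceeds only if the overlapping actor is the first found of that class.
; It swaps to the WaterConvey material as a brief warning, then hides, disables mesh collision and restores the leaf material saved at construction.
; After a longer delay it reappears with collision re-enabled.
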(event `self.ReceiveBeginPlay`)

(event `self.ReceiveActorBeginOverlap`
  (params (OtherActor :type "Actor Object Reference"))
  (if (or (or (!= OtherActor (`GameplayStatics.GetPlayerCharacter` 0)) (!= OtherActor (`GameplayStatics.GetPlayerCharacter` 1))) (or (!= OtherActor (`GameplayStatics.GetPlayerCharacter` 2)) (!= OtherActor (`GameplayStatics.GetPlayerCharacter` 3))))
    (bind _aslob_attack (castclass `/Game/Blueprints/ai/LobAttack` "/Game/Blueprints/ai/LobAttack.LobAttack_C")
      (:`then`
        (bind _outactors (`GameplayStatics.GetAllActorsOfClass` _aslob_attack))
        (if (== OtherActor (`KismetArrayLibrary.Array_Get` _outactors))
          (`self.ConveyMat`)
          (`KismetSystemLibrary.Delay` 1.6)
          (`self.RecievedLobAttack`)
          (`KismetSystemLibrary.Delay` 12.0)
          (`self.FinishLobAttack`)))
      (:`CastFailed`
        (`KismetSystemLibrary.PrintString` "double senpai fail")))))

(event `self.ReceiveTick`
  (params (DeltaSeconds :type "Float (single-precision)")))

(fn `ConveyMat`
  (`PrimitiveComponent.SetMaterial` 0 "/Game/Materials/WaterConvey.WaterConvey"))

(fn `FinishLobAttack`
  (`self.SetActorHiddenInGame` false)
  (`PrimitiveComponent.SetCollisionEnabled` (`self.StaticMesh`) "QueryAndPhysics") ; check this
)

(fn `RecievedLobAttack`
  (`self.SetActorHiddenInGame` true)
  (`PrimitiveComponent.SetCollisionEnabled` (`self.StaticMesh`) "NoCollision") ; check this
  (`PrimitiveComponent.SetMaterial` 0 (`self.OldMaterial`)))

(fn `UserConstructionScript`
  (set `self.OldMaterial` (`self.Leafmat`)))