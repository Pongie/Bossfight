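; Shared camera actor that becomes player 0's view and follows the midpoint of the outermost MyCharacter actors on X and Y.
; Each Tick it projects characters after the first to screen space, intending edge margins to trigger ZoomOut and central bands ZoomIn.
; The overlapping Y tests always choose ZoomOut inside the loop; the ZoomIn check follows loop completion.
; Curve-scaled zoom sets a clamped CamBoomLength, but the spring-arm interpolation is disconnected.
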(event `ZoomIn`
  (bind _targetarmlength (`SpringArmComponent.TargetArmLength` (`self.SpringArm`)))
  ;[1 1 1] Zoom Event Functionality
  (set `self.CamBoomLength` (`KismetMathLibrary.FClamp` (- _targetarmlength (* (`CurveFloat.GetFloatValue` (`self.ZoomCurve`) _targetarmlength) 100.0)) 300.0 1200.0)))

(event `self.ReceiveBeginPlay`
  (`PlayerController.SetViewTargetWithBlend` (`GameplayStatics.GetPlayerController` 0) self 0.0 "VTBlend_Linear" 0.0 false)
  (bind _outactors (`GameplayStatics.GetAllActorsOfClass` "/Game/Blueprints/MyCharacter.MyCharacter_C"))
  (for _index (range (+ (`KismetArrayLibrary.Array_LastIndex` _outactors) 1))
    (`KismetArrayLibrary.Array_Add` (`self.chars`) (`KismetArrayLibrary.Array_Get` _outactors _index))))

(event `ZoomOut`
  (bind _targetarmlength (`SpringArmComponent.TargetArmLength` (`self.SpringArm`)))
  ;[1 1 1] Zoom Event Functionality
  (set `self.CamBoomLength` (`KismetMathLibrary.FClamp` (+ (* (`CurveFloat.GetFloatValue` (`self.ZoomCurve`) _targetarmlength) 100.0) _targetarmlength) 400.0 1300.0)))

(event `self.ReceiveActorBeginOverlap`
  (params (OtherActor :type "Actor Object Reference")))

(event `self.ReceiveTick`
  (params (DeltaSeconds :type "Float (single-precision)"))
  (bind _chars (`self.chars`))
  (bind _chars_2 (`self.chars`))
  (bind (_x _y) (`KismetMathLibrary.BreakVector2D` (`WidgetLayoutLibrary.GetViewportSize`)))
  (bind _returnvalue (/ _y 8.0))
  (bind _returnvalue_2 (/ _x 8.0))
  (bind _returnvalue_3 (- _y _returnvalue))
  (bind _returnvalue_4 (* _returnvalue 3.0))
  (bind _returnvalue_5 (* _returnvalue_2 3.0))
  (bind _output_get (set `self.left` (`KismetArrayLibrary.Array_Get` (`self.chars`))))
  (bind _output_get_2 (set `self.right` _output_get))
  (bind _output_get_3 (set `self.top` _output_get_2))
  (set `self.bottom` _output_get_3)
  (for _index (range 1 (+ (`KismetArrayLibrary.Array_LastIndex` _chars_2) 1))
    (bind _item (`KismetArrayLibrary.Array_Get` _chars_2 _index))
    (bind _x_2 (.x (.location (`self.GetTransform` _item))))
    (bind _y_2 (.y (.location (`self.GetTransform` _item))))
    (if (< _y_2 (.y (.location (`self.GetTransform` (`self.left`)))))
      (set `self.left` _item)
      (else
        (if (> _y_2 (.y (.location (`self.GetTransform` (`self.right`)))))
          (set `self.right` _item))
        (if (> _x_2 (.x (.location (`self.GetTransform` (`self.top`)))))
          (set `self.top` _item))
        (if (< _x_2 (.x (.location (`self.GetTransform` (`self.bottom`)))))
          (set `self.bottom` _item)))))
  (`self.K2_SetActorLocation` (`KismetMathLibrary.MakeVector` (/ (+ (.x (.location (`self.GetTransform` (`self.top`)))) (.x (.location (`self.GetTransform` (`self.bottom`))))) 2.0) (/ (+ (.y (.location (`self.GetTransform` (`self.left`)))) (.y (.location (`self.GetTransform` (`self.right`))))) 2.0)))
  (for _index_2 (range 1 (+ (`KismetArrayLibrary.Array_LastIndex` _chars) 1))
    (bind (_x_3 _y_3) (`KismetMathLibrary.BreakVector2D` (`PlayerController.ProjectWorldLocationToScreen` (`GameplayStatics.GetPlayerController` _index_2) (.location (`self.GetTransform` (`KismetArrayLibrary.Array_Get` _chars _index_2))))))
    (bind _returnvalue_6 (<= _x_3 _returnvalue_2))
    ;[1 1 1] When To Zoom
    (if _returnvalue_6
      (`self.ZoomOut` :!label _label) ; should take priority
      (else
        (bind _returnvalue_7 (>= _x_3 (- _x _returnvalue_2)))
        (if _returnvalue_7
          (goto _label)
          (else
            (bind _returnvalue_8 (>= _y_3 _returnvalue_3))
            (if _returnvalue_8
              (goto _label)
              (else
                (bind _returnvalue_9 (<= _y_3 _returnvalue_3))
                (if _returnvalue_9
                  (goto _label)
                  (else
                    (if true :!label _label_2
                      (if (and (and (>= _y_3 _returnvalue_4) (<= _y_3 (- _y _returnvalue_4))) (and (!= _returnvalue_8 true) (!= _returnvalue_9 true)))
                        (`self.ZoomIn` :!label _label_3)
                        (elif (and (and (>= _x_3 _returnvalue_5) (<= _x_3 (- _x _returnvalue_5))) (and (!= _returnvalue_7 true) (!= _returnvalue_6 true)))
                          (goto _label_3)))))))))))))
  (goto _label_2))

(fn `UserConstructionScript`)