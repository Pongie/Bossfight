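; Tornado actor that knocks MyCharacter away when the player character runs into it.
; Hit and ActorBeginOverlap share one chain that casts to MyCharacter and launches it along the scaled, negated hit normal with extra lift, though only Hit supplies that normal.
; BeginPlay fetches PainCausingVolume actors without using them, Tick is empty, and move-to, waypoint and radial-force nodes are disconnected leftovers.
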(event `self.ReceiveBeginPlay`
  (`GameplayStatics.GetAllActorsOfClass` "/Script/Engine.PainCausingVolume"))

(event `self.ReceiveActorBeginOverlap`
  (params (OtherActor :type "Actor Object Reference"))
  (bind _asmy_character (cast `/Game/Blueprints/MyCharacter` (stale `self.ReceiveHit` Other) :!label _label))
  (`self.LaunchCharacter` _asmy_character (`KismetMathLibrary.MakeVector` (.x (* (stale `self.ReceiveHit` HitNormal) -400.0)) (.y (* (stale `self.ReceiveHit` HitNormal) -400.0)) (+ (.z (* (stale `self.ReceiveHit` HitNormal) -400.0)) 100.0)) false false))

(event `self.ReceiveTick`
  (params (DeltaSeconds :type "Float (single-precision)")))

(event `self.ReceiveHit`
  (params (MyComp :type "PrimitiveComponent Object Reference") (Other :type "Actor Object Reference") (OtherComp :type "PrimitiveComponent Object Reference") (bSelfMoved :type Boolean) (HitLocation :type "Object.Vector Structure") (HitNormal :type "Object.Vector Structure") (NormalImpulse :type "Object.Vector Structure") (Hit :type "EngineTypes.HitResult Structure (by ref)"))
  (goto _label))

(fn `UserConstructionScript`)