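; Inventory component that stores item actors in separate orb and utility lists and can print or drop items.
; AddOrb and AddUtility insertion-sort by Order, then Level, stacking exact matches by raising Count and destroying the incoming actor.
; DisplayItem and DropItem use a separate ItemList, which nothing here fills.
; DropItem ignores its Index, spawning a scaled-down copy of the last item near the owner and decrementing or removing that entry.
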(event `self.ReceiveTick`
  (params (DeltaSeconds :type "Float (single-precision)")))

(event `self.ReceiveInitializeComponent`)

(fn `AddOrb`
  (params (Item :type "/Game/Blueprints/Items/Item Object Reference"))
  (bind _orblist (`self.orbList`))
  (bind _orblist_2 (`self.orbList`))
  (bind _temp (`self.temp`))
  (bind _order (`/Game/Blueprints/Items/Item.order` _temp))
  (bind _level (`/Game/Blueprints/Items/Item.level` _temp))
  (`/Engine/EditorBlueprintResources/StandardMacros.IsValid` Item
    (:`Is Valid`
      (bind _output_get (set `self.temp` Item))
      (if (== (`KismetArrayLibrary.Array_Length` _orblist) 0)
        (`KismetArrayLibrary.Array_Add` _orblist _output_get :!label _label)
        (else
          (for _index (range (+ (`KismetArrayLibrary.Array_LastIndex` _orblist_2) 1))
            (bind _output_get_2 (set `self.tempIndex` _index))
            (bind _item (`KismetArrayLibrary.Array_Get` _orblist_2 _index))
            (bind _order_2 (`/Game/Blueprints/Items/Item.order` _item))
            (if (< _order _order_2)
              (`KismetArrayLibrary.Array_Insert` _orblist_2 _temp _index)
              (break)
              (elif (== _order _order_2)
                (bind _level_2 (`/Game/Blueprints/Items/Item.level` _item))
                (if (< _level _level_2)
                  (`KismetArrayLibrary.Array_Insert` _orblist_2 (`self.temp`) _index)
                  (break)
                  (elif (== _level_2 _level)
                    (bind _item_2 (`KismetArrayLibrary.Array_Get` (`self.orbList`) _index))
                    (set `/Game/Blueprints/Items/Item.count` (+ (`/Game/Blueprints/Items/Item.count` _item_2) 1) _item_2)
                    (set `self.tempIndex` (- (`self.tempIndex`) -10))
                    (`Actor.K2_DestroyActor` (`self.temp`))
                    (break))))))
          (if (== _output_get_2 (`KismetArrayLibrary.Array_LastIndex` _orblist_2))
            (goto _label)))))
    (:`Is Not Valid`
      (`KismetSystemLibrary.PrintString` "item error"))))

(fn `AddUtility`
  (params (Item :type "/Game/Blueprints/Items/Item Object Reference"))
  (bind _utilitylist (`self.utilityList`))
  (bind _utilitylist_2 (`self.utilityList`))
  (bind _utilitylist_3 (`self.utilityList`))
  (bind _temp (`self.temp`))
  (bind _order (`/Game/Blueprints/Items/Item.order` _temp))
  (bind _level (`/Game/Blueprints/Items/Item.level` _temp))
  (bind _output_get (set `self.temp` Item))
  (if (== (`KismetArrayLibrary.Array_Length` _utilitylist) 0)
    (`KismetArrayLibrary.Array_Add` _utilitylist _output_get :!label _label)
    (else
      (for _index (range (+ (`KismetArrayLibrary.Array_LastIndex` _utilitylist_2) 1))
        (bind _output_get_2 (set `self.tempIndex` _index))
        (bind _item (`KismetArrayLibrary.Array_Get` _utilitylist_2 _index))
        (bind _order_2 (`/Game/Blueprints/Items/Item.order` _item))
        (if (< _order _order_2)
          (`KismetArrayLibrary.Array_Insert` _utilitylist_2 _temp _index)
          (break)
          (elif (== _order _order_2)
            (bind _level_2 (`/Game/Blueprints/Items/Item.level` _item))
            (if (< _level _level_2)
              (`KismetArrayLibrary.Array_Insert` _utilitylist_3 (`self.temp`) _index)
              (break)
              (elif (== _level_2 _level)
                (bind _item_2 (`KismetArrayLibrary.Array_Get` _utilitylist_3 _index))
                (set `/Game/Blueprints/Items/Item.count` (+ (`/Game/Blueprints/Items/Item.count` _item_2) 1) _item_2)
                (set `self.tempIndex` (- (`self.tempIndex`) -10))
                (`Actor.K2_DestroyActor` (`self.temp`))
                (break))))))
      (if (== _output_get_2 (`KismetArrayLibrary.Array_LastIndex` _utilitylist))
        (goto _label)))))

(fn `DisplayItem`
  (for _index (range (+ (`KismetArrayLibrary.Array_LastIndex` (`self.itemList`)) 1))
    (bind _item (`KismetArrayLibrary.Array_Get` (`self.itemList`) _index))
    (`KismetSystemLibrary.PrintText` (`KismetTextLibrary.Conv_StringToText` (`KismetStringLibrary.Concat_StrStr` (`KismetStringLibrary.Concat_StrStr` (`KismetStringLibrary.Concat_StrStr` (`KismetStringLibrary.Concat_StrStr` (`/Game/Blueprints/Items/Item.name` _item) " ") (`KismetStringLibrary.Conv_IntToString` (`/Game/Blueprints/Items/Item.level` _item))) "x") (`KismetStringLibrary.Conv_IntToString` (`/Game/Blueprints/Items/Item.count` _item)))))))

(fn `DropItem`
  (params (Index :type Integer))
  (bind _returnvalue (`self.GetOwner`))
  (bind _itemlist (`self.itemList`))
  (bind _itemlist_2 (`self.itemList`))
  (bind _returnvalue_2 (`KismetArrayLibrary.Array_LastIndex` _itemlist))
  (bind _item (`KismetArrayLibrary.Array_Get` _itemlist_2 _returnvalue_2))
  (bind _count (`/Game/Blueprints/Items/Item.count` _item))
  (bind _asactor (castclass `Actor` (`GameplayStatics.GetObjectClass` (`KismetArrayLibrary.Array_Get` _itemlist _returnvalue_2))))
  (`|SpawnActorFromClass` _asactor (`KismetMathLibrary.MakeTransform` (+ (`Actor.K2_GetActorLocation` _returnvalue) (100.0 0.0 0.0)) (`Actor.K2_GetActorRotation` _returnvalue) (0.3 0.3 0.3)))
  (set `/Game/Blueprints/Items/Item.level` (`/Game/Blueprints/Items/Item.level` _item) _item)
  (if (> _count 1)
    (set `/Game/Blueprints/Items/Item.count` (- _count 1) _item)
    (else
      (`KismetArrayLibrary.Array_Remove` _itemlist_2 _returnvalue_2))))