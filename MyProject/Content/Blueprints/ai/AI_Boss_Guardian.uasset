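; Guardian boss AI Blueprint that fires three attacks when EnemyFoundEvent runs.
; Parallel delayed branches spawn a lob projectile, a particle spore volley that is later destroyed, and a rock wave attack, each with a sound.
; A forward box trace sets the lob's initial speed from hit distance.
; Tick feeds a gated, unfinished debug trajectory preview that line-traces ballistic segments, marked by the author to disregard.
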(event Custom|Draw%20Trajectory
  (bind _returnvalue (Pawn|GetControlRotation :!class /Script/Engine.Pawn))
  (bind _returnvalue_2 (Transformation|GetActorLocation))
  (bind _returnvalue_3 (Math|Vector|GetForwardVector _returnvalue))
  (bind _returnvalue_4 (* _returnvalue_3 2e+02))
  (bind _returnvalue_5 (+ _returnvalue_2 _returnvalue_4))
  (bind _returnvalue_6 (- _returnvalue_5 "0.000000, 0,100.000000"))
  ;[1 1 1] Trying to draw trajectory, disregard
  (Variables|Default|Setstartloc _returnvalue_6)
  (Variables|Default|SetinitVel (Math|Transform|TransformDirection (Math|Transform|MakeTransform _returnvalue_6 (Transformation|GetActorRotation) "1.000000,1.000000,1.000000") (Variables|Default|Getinitlocalvelocity)))
  (bind _index (Utilities|FlowControl|ForLoopwithBreak 0 (Math|Float|Floor (/ (Variables|Default|GetTrajPathLifetime) (Variables|Default|GetTimeInterval))))
    (:LoopBody
      (bind (_point_1 _point_2) (CallFunction|GetSegmentatTime (Variables|Default|Getstartloc) (Variables|Default|GetinitVel) "0, 0,-5000.000000" (* _index (Variables|Default|GetTimeInterval)) (* (+ _index 1) (Variables|Default|GetTimeInterval))))
      (bind _returnvalue_7 (Collision|LineTraceByChannel _point_1 _point_2 "TraceTypeQuery1" true 0 "ForOneFrame"))
      (CallFunction|VisualizeSegment _point_1 _point_2 "NewEnumerator0")
      (if _returnvalue_7
        (CallFunction|BreakDrawLoop)))))

(event Custom|BreakDrawLoop
  ;[1 1 1] Trying to draw trajectory, disregard
  (Utilities|FlowControl|ForLoopwithBreak 0 (Math|Float|Floor (/ (Variables|Default|GetTrajPathLifetime) (Variables|Default|GetTimeInterval)))) ; enters at Break
)

(event EventBeginPlay
  (|CallParentFunction)
  (Variables|Default|SetDrawtype "NewEnumerator0"))

(event EventActorBeginOverlap
  (params (OtherActor :type Actor%20Object%20Reference)))

(event EventTick
  (params (DeltaSeconds :type Float%20%28single-precision%29))
  (|CallParentFunction 0.0)
  (Utilities|FlowControl|Gate true :!label _label
    (:Exit
      (CallFunction|DrawTrajectory)
      (Utilities|FlowControl|Delay 2.0)
      (goto _label Close))))

(event EventEnemyFoundEvent
  (bind _returnvalue (Pawn|GetControlRotation :!class /Script/Engine.Pawn))
  (bind _returnvalue_2 (Transformation|GetActorLocation))
  (bind _returnvalue_3 (Math|Vector|GetForwardVector _returnvalue))
  (bind _returnvalue_4 (* _returnvalue_3 2e+02))
  (bind _returnvalue_5 (+ _returnvalue_2 _returnvalue_4))
  (Utilities|FlowControl|Sequence
    (:then_0
      ;[1 1 1] Attack 1
      (Utilities|FlowControl|Delay 6.0)
      (Game|SpawnActorfromClass "/Game/Blueprints/bossattacks/WaveAttackRock.WaveAttackRock_C" (Math|Transform|MakeTransform (- (+ (Transformation|GetActorLocation) (* (Math|Vector|GetForwardVector (Pawn|GetControlRotation :!class /Script/Engine.Pawn)) 2e+02)) "0, 0,90.000000") (Transformation|GetActorRotation) "1.000000,1.000000,1.000000") false 0)
      (Audio|PlaySoundatLocation "/Game/Sounds/wave_attack_rock.wave_attack_rock" "0, 0, 0"))
    (:then_1
      ;[1 1 1] Attack 2
      (Utilities|FlowControl|Delay 3.0)
      (bind _outhit (Collision|BoxTraceByChannel _returnvalue_5 (* _returnvalue_3 3.33e+03) "64.000000,64.000000,64.000000" "0, 0, 0" "TraceTypeQuery1" true 0 "None"))
      (bind _returnvalue_6 (Game|SpawnActorfromClass "/Game/Blueprints/bossattacks/LobAttack.LobAttack_C" (Math|Transform|MakeTransform (- _returnvalue_5 "0.000000, 0,100.000000") (Transformation|GetActorRotation) "1.000000,1.000000,1.000000") true 0))
      (Audio|PlaySoundatLocation "/Game/Sounds/lob_attack.lob_attack" "0, 0, 0")
      (bind _output_get (Variables|/Script/Engine.ProjectileMovementComponent|SetInitialSpeed (Variables|/Game/Blueprints/bossattacks/LobAttack.LobAttack_C|GetProjectileMovement _returnvalue_6) (Math|Vector|VectorLength (- _returnvalue_5 (.Location (Collision|BreakHitResult _outhit)))))))
    (:then_2
      ;[1 1 1] Attack3
      (Utilities|FlowControl|Delay 4.0)
      (bind _returnvalue_7 (Game|SpawnActorfromClass "/Game/Blueprints/bossattacks/ProjVolley.ProjVolley_C" (Math|Transform|MakeTransform (+ "0, 0, 0" (Transformation|GetActorLocation) (Math|Vector|GetForwardVector (Pawn|GetControlRotation :!class /Script/Engine.Pawn))) (Transformation|GetActorRotation) "1.000000,1.000000,1.000000") true 0))
      (Audio|PlaySoundatLocation "/Game/Sounds/spore_spray.spore_spray" "0, 0, 0")
      (Effects|Components|ParticleSystem|SetVectorParameter (Variables|/Game/Blueprints/bossattacks/ProjVolley.ProjVolley_C|GetParticleSystem _returnvalue_7) "InitRot" (Math|Vector|GetForwardVector (Pawn|GetControlRotation :!class /Script/Engine.Pawn)))
      (Effects|Components|ParticleSystem|SetVectorParameter (Variables|/Game/Blueprints/bossattacks/ProjVolley.ProjVolley_C|GetParticleSystem _returnvalue_7) "VelocityShot" (+ "-40.000000,0.000000,-500.000000" (Transformation|GetActorLocation) (Math|Vector|GetForwardVector (Pawn|GetControlRotation :!class /Script/Engine.Pawn))))
      (Utilities|FlowControl|Delay 4.2)
      (Actor|DestroyActor _returnvalue_7))))

(fn ConstructionScript
  (|CallParentFunction)
  (Rendering|Material|SetMaterial 0 "/Game/Outsourced/Meshes/Nature_Guard_ZRemesh_blinn.Nature_Guard_ZRemesh_blinn"))

(fn GetSegmentatTime
  (params (Start%20Loc :type Vector :default "0, 0, 0") (Init%20Velocity :type Vector :default "0, 0, 0") (Gravity :type Vector :default "0, 0, 0") (Time%201 :type Float%20%28single-precision%29 :default 0.0) (Time%202 :type Float%20%28single-precision%29 :default 0.0))
  (return (+ Start%20Loc (* Init%20Velocity Time%201) (* Gravity (* Time%201 Time%202 0.5))) (+ Start%20Loc (* Init%20Velocity Time%202) (* Gravity (* Time%202 Time%202 0.5)))))

(fn VisualizeSegment
  (params (Point%201 :type Vector :default "0, 0, 0") (Point%202 :type Vector :default "0, 0, 0") (Ty :type DrawingType%20Enum :default "NewEnumerator0"))
  (LocalVariables|Setp1 Point%201)
  (LocalVariables|Setp2 Point%202)
  (switch Utilities|FlowControl|Switch|SwitchonDrawingType Ty
    (:NewEnumerator0
      (Rendering|Debug|DrawDebugLine (LocalVariables|Getp1) (LocalVariables|Getp2) "(R=0.000000,G=1.000000,B=0.113013,A=1.000000)" 0.0 3.0))
    (:NewEnumerator1)))