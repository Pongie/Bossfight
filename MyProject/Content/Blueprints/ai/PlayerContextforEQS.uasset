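; EQS context that supplies the player as a single actor, used by the FindHidingSpot query to check visibility.
; For an EQS testing pawn querier, it returns the first MyCharacter found in the world, which allows editor previews.
; For other queriers, it returns the PlayerEnemy stored on their Runnier_AI_CON controller.
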(fn ProvideSingleActor
  (params (QuerierActor :type Actor%20Object%20Reference))
  ;[1 1 1] With the EQS FindHidingSpot, we are checking to see the visibility of an actor.  Here we filter the Results of what actor we find
  (Utilities|Casting|CastToEQSTestingPawn QuerierActor
    (:then
      (bind _outactors (Actor|GetAllActorsOfClass "/Game/Blueprints/MyCharacter.MyCharacter_C"))
      (LocalVariables|SetTempplayer (Utilities|Array|Get(acopy) _outactors)))
    (:CastFailed
      (bind _returnvalue (AI|GetAIController QuerierActor))
      (if (!= _returnvalue 0)
        (bind _asrunnier_ai_con (Utilities|Casting|CastToRunnier_AI_CON _returnvalue)
          (:then
            (LocalVariables|SetTempplayer (Variables|/Game/Blueprints/ai/Runnier_AI_CON.Runnier_AI_CON_C|GetPlayer%28Enemy%29 _asrunnier_ai_con)))
          (:CastFailed
            _)))))
  (return (LocalVariables|GetTempplayer)))