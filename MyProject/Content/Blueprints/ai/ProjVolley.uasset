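; Particle-based volley hazard, filed under AI, that deals damage over time to up to four player characters cached on BeginPlay.
; A particle collision traces from Origin to the impact point and damages a player it hits.
; A hard-coded chain of one-second Delays repeats the damage while the shared Inradius flag holds.
; Any Detect end-overlap clears that flag, as its index check compares the value to itself.
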(event `self.ReceiveBeginPlay`
  (bind _asmy_character (cast `/Game/Blueprints/MyCharacter` (`GameplayStatics.GetPlayerCharacter` 0))
    (:`then`
      (bind _output_get (set `self.p1` _asmy_character)))
    (:`CastFailed`
      _))
  (bind _asmy_character_2 (cast `/Game/Blueprints/MyCharacter` (`GameplayStatics.GetPlayerCharacter` 1))
    (:`then`
      (bind _output_get_2 (set `self.p2` _asmy_character_2)))
    (:`CastFailed`
      _))
  (bind _asmy_character_3 (cast `/Game/Blueprints/MyCharacter` (`GameplayStatics.GetPlayerCharacter` 2))
    (:`then`
      (bind _output_get_3 (set `self.p3` _asmy_character_3)))
    (:`CastFailed`
      _))
  (bind _asmy_character_4 (cast `/Game/Blueprints/MyCharacter` (`GameplayStatics.GetPlayerCharacter` 3)))
  (bind _output_get_4 (set `self.p4` _asmy_character_4)))

(event `self.ReceiveTick`
  (params (DeltaSeconds :type "Float (single-precision)")))

(event `self.ParticleSystem.OnParticleCollide`
  (params (EventName :type Name) (EmitterTime :type "Float (single-precision)") (ParticleTime :type Integer) (Location :type "Object.Vector Structure") (Velocity :type "Object.Vector Structure") (Direction :type "Object.Vector Structure") (Normal :type "Object.Vector Structure") (BoneName :type Name))
  (bind _damage (`self.Damage`))
  (bind _outhit (`KismetSystemLibrary.LineTraceSingle` :`Start` (`SceneComponent.K2_GetComponentLocation` (`self.origin`)) :`End` Location :`TraceChannel` "TraceTypeQuery1" :`bTraceComplex` true :`DrawDebugType` "ForOneFrame"))
  (bind (_bblockinghit _time _location _normal _impactpoint _impactnormal _physmat _hitactor) (`GameplayStatics.BreakHitResult` _outhit))
  (if (or (or (== _hitactor (stale `self.ReceiveBeginPlay` _output_get_3)) (== _hitactor (stale `self.ReceiveBeginPlay` _output_get_4))) (or (== _hitactor (stale `self.ReceiveBeginPlay` _output_get)) (== _hitactor (stale `self.ReceiveBeginPlay` _output_get_2))))
    (bind _output_get (set `self.inradius` true))
    (`GameplayStatics.ApplyDamage` _hitactor _damage)
    (`KismetSystemLibrary.Delay` 1.0)
    (if _output_get
      (`GameplayStatics.ApplyDamage` _hitactor _damage)
      (`KismetSystemLibrary.Delay` 1.0)
      (if _output_get
        (`GameplayStatics.ApplyDamage` _hitactor _damage)
        (`KismetSystemLibrary.Delay` 1.0)
        (if _output_get
          (`GameplayStatics.ApplyDamage` _hitactor _damage)
          (`KismetSystemLibrary.Delay` 1.0)
          (if _output_get
            (`GameplayStatics.ApplyDamage` _hitactor _damage)
            (`KismetSystemLibrary.Delay` 1.0)
            (if _output_get
              (`GameplayStatics.ApplyDamage` _hitactor _damage)
              (`KismetSystemLibrary.Delay` 1.0)
              (if _output_get
                (`GameplayStatics.ApplyDamage` _hitactor _damage)
                (`KismetSystemLibrary.Delay` 1.0)
                (if _output_get
                  (`GameplayStatics.ApplyDamage` _hitactor _damage)
                  (`KismetSystemLibrary.Delay` 1.0)
                  (if _output_get
                    (`GameplayStatics.ApplyDamage` _hitactor _damage)))))))))))

(event `self.detect.OnComponentBeginOverlap`
  (params (OtherActor :type "Actor Object Reference") (OtherComp :type "PrimitiveComponent Object Reference") (OtherBodyIndex :type Integer) (bFromSweep :type Boolean) (SweepResult :type "EngineTypes.HitResult Structure (by ref)")))

(event `self.detect.OnComponentEndOverlap`
  (params (OtherActor :type "Actor Object Reference") (OtherComp :type "PrimitiveComponent Object Reference") (OtherBodyIndex :type Integer))
  (if (== (stale `self.detect.OnComponentBeginOverlap` OtherBodyIndex) OtherBodyIndex)
    (set `self.inradius` false)))

(event `self.ParticleSystem.OnComponentHit`
  (params (OtherActor :type "Actor Object Reference") (OtherComp :type "PrimitiveComponent Object Reference") (NormalImpulse :type "Object.Vector Structure") (Hit :type "EngineTypes.HitResult Structure (by ref)"))
  (`KismetSystemLibrary.PrintString` "senpai attack" :!label _label))

(event `self.ParticleSystem.OnComponentBeginOverlap`
  (params (OtherActor :type "Actor Object Reference") (OtherComp :type "PrimitiveComponent Object Reference") (OtherBodyIndex :type Integer) (bFromSweep :type Boolean) (SweepResult :type "EngineTypes.HitResult Structure (by ref)"))
  (goto _label))

(fn `UserConstructionScript`)