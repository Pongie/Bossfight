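; Boss 1 enemy character that chases players, can be stunned, flashes when hit and is destroyed at zero hitpoints.
; Tick zeroes walk speed while stunned, with a timer to clear it.
; A health threshold triggers a one-time enrage camera cut, briefly toggling player input, collision and AI possession.
; Finding an enemy schedules a random-delay aggro swap that writes a sphere-trace hit to the blackboard's EnemyActor.
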(event `self.ReceiveBeginPlay`
  ;[1 1 1] Initialize
  (bind _asmy_character (castclass `/Game/Blueprints/MyCharacter` "/Game/Blueprints/MyCharacter.MyCharacter_C"))
  (bind _outactors (`GameplayStatics.GetAllActorsOfClass` _asmy_character))
  (bind _asgame_data (cast `/Game/Blueprints/GameData` (`GameplayStatics.GetGameInstance`)))
  (for _index (range (`/Game/Blueprints/GameData.playerCount` _asgame_data))
    (bind _asmy_character_2 (cast `/Game/Blueprints/MyCharacter` (`KismetArrayLibrary.Array_Get` _outactors _index)))
    (`KismetArrayLibrary.Array_Add` (`self.PlayerRef`) _asmy_character_2)
    (bind _outactors_2 (`GameplayStatics.GetAllActorsOfClass` "/Game/Blueprints/CameraFocusActor.CameraFocusActor_C"))
    (cast `/Game/Blueprints/CameraFocusActor` (`KismetArrayLibrary.Array_Get` _outactors_2))))

(event `stunTimer`
  ;[1 1 1] Speed
  (set `self.isStunned` false))

(event `self.ReceiveTick`
  (params (DeltaSeconds :type "Float (single-precision)"))
  (bind _charactermovement (`self.CharacterMovement`))
  ;[1 1 1] Speed
  (if (`self.isStunned`)
    (set `CharacterMovementComponent.MaxWalkSpeed` 0.0 _charactermovement)
    (`KismetSystemLibrary.K2_SetTimer` null "stunTimer" 5.0)
    (else
      (set `CharacterMovementComponent.MaxWalkSpeed` (* (`self.speedRate`) (`self.SpeedVariable`)) _charactermovement))))

(event `self.ReceiveActorBeginOverlap`
  (params (OtherActor :type "Actor Object Reference")))

(event `self.ReceiveAnyDamage`
  (params (Damage :type "Float (single-precision)") (DamageType :type "DamageType Object Reference") (InstigatedBy :type "Controller Object Reference") (DamageCauser :type "Actor Object Reference"))
  (bind _returnvalue (`GameplayStatics.GetPlayerController` 0))
  (bind _maxhitpoints (`self.Maxhitpoints`))
  (bind _springarm (`self.SpringArm`))
  (if (`self.enraged`)
    ;[1 1 1] When Hit Recieved
    (bind _output_get (set `self.Hitpoints` (- (`self.Hitpoints`) Damage) :!label _label))
    ;[1 1 1] When Hit Successful
    (`GameplayStatics.PlaySoundAtLocation` null)
    (`PrimitiveComponent.SetMaterial` 0 "/Game/Materials/HitFlash.HitFlash")
    (`KismetSystemLibrary.Delay` 0.08)
    (`PrimitiveComponent.SetMaterial` (`self.Mesh`) 0 (`self.OriginMaterialRef`))
    ;;[1 1 1] Check if Dead
    (if (<= _output_get 0.0)
      (`GameplayStatics.PlaySoundAtLocation` "/Game/Sounds/boss_death.boss_death")
      (`self.K2_DestroyActor`))
    (else
      ;[1 1 1] Matinee Update
      (if (<= (* (/ (`self.Hitpoints`) _maxhitpoints) 100.0) (- _maxhitpoints (/ _maxhitpoints 4.0)))
        (set `self.enraged` true)
        (bind _output_get_2 (set `self.OldViewRef` (`Controller.GetViewTarget` _returnvalue)))
        (`PlayerController.SetViewTargetWithBlend` _returnvalue self 0.0 "VTBlend_EaseInOut" 0.0 false)
        (bind _asgame_data (cast `/Game/Blueprints/GameData` (`GameplayStatics.GetGameInstance`)))
        (bind _returnvalue_2 (- (`/Game/Blueprints/GameData.playerCount` _asgame_data) 1))
        (for _index (range (+ _returnvalue_2 1))
          (bind _returnvalue_3 (`GameplayStatics.GetPlayerController` _index))
          (`self.DisableInput` (`Controller.K2_GetPawn` _returnvalue_3) _returnvalue_3)
          (`self.DisableInput` (`KismetArrayLibrary.Array_Get` (`self.PlayerRef`) _index) _returnvalue_3)
          (`PrimitiveComponent.SetCollisionEnabled` (`KismetArrayLibrary.Array_Get` (`self.PlayerRef`) _index) "NoCollision"))
        (bind _returnvalue_4 (`AIBlueprintHelperLibrary.GetAIController` self))
        (`Controller.UnPossess` _returnvalue_4)
        ;;[1 1 1] Camera Logic
        (bind _returnvalue_5 (`SceneComponent.GetRelativeTransform` _springarm))
        (`SceneComponent.K2_AddRelativeRotation` _springarm (`KismetMathLibrary.MakeRot` (+ (.x (`KismetMathLibrary.Conv_RotatorToVector` (.rotation _returnvalue_5))) 90.0) (.y (`KismetMathLibrary.Conv_RotatorToVector` (.rotation _returnvalue_5))) (.z (`KismetMathLibrary.Conv_RotatorToVector` (.rotation _returnvalue_5)))) false)
        (for _index_2 (range (+ _returnvalue_2 1))
          (bind _returnvalue_6 (`GameplayStatics.GetPlayerController` _index_2))
          (`self.EnableInput` (`Controller.K2_GetPawn` _returnvalue_6) _returnvalue_6)
          (`PrimitiveComponent.SetCollisionEnabled` (`KismetArrayLibrary.Array_Get` (`self.PlayerRef`) _index_2) "QueryAndPhysics"))
        (`Controller.Possess` _returnvalue_4 self)
        (`PlayerController.SetViewTargetWithBlend` (`GameplayStatics.GetPlayerController` 0) _output_get_2 0.5 "VTBlend_EaseIn" (`CurveFloat.GetFloatValue` (`self.CurveFloat`) 2.0) false)
        (else
          (goto _label))))))

(event `EnemyLost_Event`
  ;[1 1 1] Stop Attack
  (add `self.EnemyLost` (delegate `EnemyLost_Event`))
  (`KismetSystemLibrary.PrintString` "Boss Disengage"))

(event `EnemyFound_Event`
  ;[1 1 1] Attack
  (if (`self.ResetTimer`)
    (`KismetSystemLibrary.K2_SetTimer` null "AggroSwap" (`KismetMathLibrary.RandomFloatInRange` 7.0 17.0))
    (set `self.ResetTimer` false)))

(event `AggroSwap`
  (bind _playerref (`self.PlayerRef`))
  (bind _enemyactor (`self.EnemyActor`))
  (bind _returnvalue (`AIBlueprintHelperLibrary.GetBlackboard` self))
  ;[1 1 1] Aggro Swap
  (set `self.ResetTimer` true)
  (bind _outhit (`KismetSystemLibrary.SphereTraceSingle_NEW` :`End` (0.0 0.0 111.0) :`Radius` 4440.0 :`TraceChannel` "TraceTypeQuery1" :`bTraceComplex` true :`DrawDebugType` "ForOneFrame"))
  (for _index (range (`KismetArrayLibrary.Array_Length` _playerref))
    (bind (_bblockinghit _time _location _normal _impactpoint _impactnormal _physmat _hitactor) (`GameplayStatics.BreakHitResult` _outhit))
    (if (== _hitactor (`KismetArrayLibrary.Array_Get` _playerref _index))
      (if (!= _hitactor (`BlackboardComponent.GetValueAsObject` _returnvalue _enemyactor))
        (break))))
  (`BlackboardComponent.SetValueAsObject` _returnvalue _enemyactor _hitactor))

(fn `UserConstructionScript`)