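; LobAttack is a projectile actor, apparently a lobbed boss attack, that explodes on hit.
; Hit applies full radial damage around itself, spawns an explosion emitter and destroys the actor.
; BeginPlay finds AI_Boss1 and runs a debug line trace from its forward vector, used as a position, to a fixed point.
; Logic to adjust projectile gravity by distance to the traced actor is disconnected and never runs.
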(event `self.ReceiveActorBeginOverlap`
  (params (OtherActor :type "Actor Object Reference")))

(event `self.ReceiveHit`
  (params (MyComp :type "PrimitiveComponent Object Reference") (Other :type "Actor Object Reference") (OtherComp :type "PrimitiveComponent Object Reference") (bSelfMoved :type Boolean) (HitLocation :type "Object.Vector Structure") (HitNormal :type "Object.Vector Structure") (NormalImpulse :type "Object.Vector Structure") (Hit :type "EngineTypes.HitResult Structure (by ref)"))
  (`GameplayStatics.ApplyRadialDamage` :`BaseDamage` 15.0 :`Origin` (`self.K2_GetActorLocation`) :`DamageRadius` 1000.0 :`bDoFullDamage` true)
  (`KismetSystemLibrary.PrintString` "radial damage applied")
  (`GameplayStatics.SpawnEmitterAtLocation` "/Game/StarterContent/Particles/P_Explosion.P_Explosion" HitLocation)
  (`self.K2_DestroyActor`))

(event `self.ReceiveBeginPlay`
  (cast `/Game/Blueprints/MyCharacter` (`GameplayStatics.GetPlayerCharacter` 0))
  (bind _outactors (`GameplayStatics.GetAllActorsOfClass` "/Game/Blueprints/ai/AI_Boss1.AI_Boss1_C"))
  (bind _asai_boss_1 (cast `/Game/Blueprints/ai/AI_Boss1` (`KismetArrayLibrary.Array_Get` _outactors))
    (:`then`
      _)
    (:`CastFailed`
      (`KismetSystemLibrary.PrintString` "liar liar senpai on fire")))
  (bind _outhit (`KismetSystemLibrary.LineTraceSingle` :`Start` (`KismetMathLibrary.GetForwardVector` (.rotation (`self.GetTransform` _asai_boss_1))) :`End` (2000.0 0.0 0.0) :`TraceChannel` "TraceTypeQuery1" :`DrawDebugType` "ForOneFrame")))

(fn `UserConstructionScript`)