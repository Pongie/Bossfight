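; AI rock wave attack actor that advances along its forward vector in repeated strikes, then destroys itself when its count runs out.
; Each Tick-driven step, gated by a Ready flag around latent delays, spawns an enlarged ripple warning, then a rock spike.
; It then applies full radial damage, ignoring AI_Boss1 actors, triples the damage radius and moves forward for the next strike.
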(event `self.ReceiveBeginPlay`
  (set `self.conveyance` "/Game/Outsourced/Effects/2ndt/P_Impact_Ripple.P_Impact_Ripple")
  (set `self.pillar` "/Game/Outsourced/Effects/Rockspike.Rockspike"))

(event `self.ReceiveActorBeginOverlap`
  (params (OtherActor :type "Actor Object Reference")))

(event `self.ReceiveTick`
  (params (DeltaSeconds :type "Float (single-precision)"))
  (bind _returnvalue (`self.K2_GetActorLocation`))
  (bind _returnvalue_2 (`self.K2_GetActorRotation`))
  (if (== (`self.count`) 0)
    (`self.K2_DestroyActor`)
    (elif (`self.ready`)
      (set `self.ready` false)
      (bind _returnvalue_3 (`GameplayStatics.SpawnEmitterAtLocation` (`self.conveyance`) _returnvalue _returnvalue_2))
      (`KismetSystemLibrary.Delay` 0.8)
      (`SceneComponent.SetWorldScale3D` _returnvalue_3 (`KismetMathLibrary.MakeVector` (* (.x (`SceneComponent.K2_GetComponentScale` _returnvalue_3)) 2.5) (* (.y (`SceneComponent.K2_GetComponentScale` _returnvalue_3)) 2.5) (.z (`SceneComponent.K2_GetComponentScale` _returnvalue_3))))
      (bind _returnvalue_4 (`GameplayStatics.SpawnEmitterAtLocation` (`self.pillar`) _returnvalue _returnvalue_2))
      (`SceneComponent.SetWorldScale3D` _returnvalue_4 (`KismetMathLibrary.MakeVector` (* (.x (`SceneComponent.K2_GetComponentScale` _returnvalue_4)) 2.5) (* (.y (`SceneComponent.K2_GetComponentScale` _returnvalue_4)) 2.5) (.z (`SceneComponent.K2_GetComponentScale` _returnvalue_4))))
      (`KismetSystemLibrary.Delay` 0.2)
      (bind _outactors (`GameplayStatics.GetAllActorsOfClass` "/Game/Blueprints/ai/AI_Boss1.AI_Boss1_C"))
      (`GameplayStatics.ApplyRadialDamage` (`self.damage`) _returnvalue (`self.radius`) null _outactors null null true)
      (set `self.radius` (* (`self.radius`) 3.0))
      (set `self.count` (- (`self.count`) 1))
      (`self.K2_SetActorLocation` (+ (`self.K2_GetActorLocation`) (* (`KismetMathLibrary.GetForwardVector` _returnvalue_2) (`self.movementDist`))))
      (set `self.ready` true))))

(fn `UserConstructionScript`)