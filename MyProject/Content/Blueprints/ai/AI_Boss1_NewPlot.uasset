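; Boss 1 AI character that attacks players with wave, melee and bounce attacks, plus an omnidirectional attack actor spawned at BeginPlay.
; EnemyFound_Event fires a delayed fire wave, cooldown-gated melee with AIMoveTo chasing, and randomly offset bounce projectiles.
; A looping timer with a randomized interval sphere-traces to swap the blackboard EnemyActor when multiple players exist.
; Teleport slam, radial blast, spear rush and projectile homing are disconnected, unfinished logic.
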(event `self.ReceiveBeginPlay`
  (`parent.ReceiveBeginPlay`)
  ;[1 1 1] init
  (bind _asmy_game_instance (cast `/Game/Blueprints/MyGameInstance` (`GameplayStatics.GetGameInstance`)))
  (`KismetSystemLibrary.K2_SetTimer` null "AggroSwap" (`KismetMathLibrary.RandomFloatInRange` 7.0 17.0) true)
  (bind _returnvalue (`|SpawnActorFromClass` "/Game/Blueprints/bossattacks/Omnidirection_attack.Omnidirection_attack_C" (`KismetMathLibrary.MakeTransform` (0.0 0.0 0.0)) true self)))

(event `self.ReceiveActorBeginOverlap`
  (params (OtherActor :type "Actor Object Reference")))

(event `self.ReceiveTick`
  (params (DeltaSeconds :type "Float (single-precision)"))
  (`parent.ReceiveTick` 0.0))

(event `EnemyFound_Event`
  (bind _returnvalue (`self.K2_GetActorRotation`))
  (bind _item (`KismetArrayLibrary.Array_Get` (`self.GetOverlappingActors` "/Game/Blueprints/MyCharacter.MyCharacter_C")))
  (bind _returnvalue_2 (- (+ (`self.K2_GetActorLocation`) (* (`KismetMathLibrary.GetForwardVector` (`self.GetControlRotation`)) 200.0)) (0.0 0.0 90.0)))
  (bind _x (.x _returnvalue_2))
  (bind _y (.y _returnvalue_2))
  (bind _z (.z _returnvalue_2))
  (`|ExecutionSequence`
    (:`then_0`
      ;[1 1 1] Attack 1
      (`KismetSystemLibrary.Delay` 2.0)
      (`|SpawnActorFromClass` "/Game/Blueprints/bossattacks/WaveAttackFire.WaveAttackFire_C" (`KismetMathLibrary.MakeTransform` (- (+ (`self.K2_GetActorLocation`) (* (`KismetMathLibrary.GetForwardVector` (`self.GetControlRotation`)) 200.0)) (0.0 0.0 90.0)) (`self.K2_GetActorRotation`) (1.0 1.0 1.0)))
      (`GameplayStatics.PlaySoundAtLocation` "/Game/Sounds/wave_attack_fire_3.wave_attack_fire_3"))
    (:`then_1`
      ;[1 1 1] Melee
      (if (not (!= _item null)) :!label _label
        (`|AIMoveTo` self (`self.K2_GetActorLocation` _item) _item 2.0
          (:`OnSuccess`
            _)
          (:`OnFail`
            (goto _label))))
      (`/Engine/EditorBlueprintResources/StandardMacros.CompareFloat` (`self.coolDownM`) (`KismetSystemLibrary.GetGameTimeInSeconds`)
        (:`<`
          (`SkeletalMeshComponent.PlayAnimation` (`self.Mesh`) "/Game/Outsourced/Meshes/Mixamo_Maw/Anims/Maw_J_Laygo_Sword_Swing.Maw_J_Laygo_Sword_Swing" false)
          (`GameplayStatics.ApplyDamage` (`KismetArrayLibrary.Array_Get` (`PrimitiveComponent.GetOverlappingActors` self "/Game/Blueprints/MyCharacter.MyCharacter_C")) 6.0)
          (set `self.coolDownM` (+ (`KismetSystemLibrary.GetGameTimeInSeconds`) 0.8))
          (if (>= (`KismetMathLibrary.RandomFloatInRange` 0.0 100.0) 40.0)
            (`KismetSystemLibrary.Delay` 0.2)
            (goto _label)))))
    (:`then_2`
      (if true
        (`/Engine/EditorBlueprintResources/StandardMacros.CompareFloat` (`self.coolDownB`) (`KismetSystemLibrary.GetGameTimeInSeconds`)
          (:`<`
            (if (>= (`KismetMathLibrary.RandomFloatInRange` 0.0 100.0) 50.0)
              (bind _returnvalue_3 (`|SpawnActorFromClass` "/Game/Blueprints/bossattacks/Bounce_attack.Bounce_attack_C" (`KismetMathLibrary.MakeTransform` (`KismetMathLibrary.MakeVector` (+ (`KismetMathLibrary.RandomFloatInRange` 0.0 200.0) _x) _y _z) _returnvalue (1.0 1.0 1.0)) true))
              (else
                ;[1 1 1] Bounce Attack
                (bind _returnvalue_4 (`|SpawnActorFromClass` "/Game/Blueprints/bossattacks/Bounce_attack.Bounce_attack_C" (`KismetMathLibrary.MakeTransform` (`KismetMathLibrary.MakeVector` (- _x (`KismetMathLibrary.RandomFloatInRange` 0.0 200.0)) _y _z) _returnvalue (1.0 1.0 1.0)) true))))
            (bind _outhit (`KismetSystemLibrary.LineTraceSingle` _returnvalue_2 (`SceneComponent.K2_GetComponentLocation` (`KismetArrayLibrary.Array_Get` (`self.PlayerRef`) (`KismetMathLibrary.RandomIntegerInRange` 0 (- (`GameMode.NumPlayers` (`GameplayStatics.GetGameMode`)) 1)))) "TraceTypeQuery1" true))
            (if true
              (if (>= (`KismetMathLibrary.RandomFloatInRange` 0.0 100.0) 30.0)
                (set `self.coolDownB` (+ (`KismetSystemLibrary.GetGameTimeInSeconds`) 0.45))))))))))

(event `ReceiveActorBeginOverlap_Copy`
  (params (OtherActor :type "Actor Object Reference")))

(event `AggroSwap`
  (bind _playerref (`self.PlayerRef`))
  (bind _enemyactor (`self.EnemyActor`))
  (bind _returnvalue (`AIBlueprintHelperLibrary.GetBlackboard` self))
  ;[1 1 1] Aggro Swap
  (`KismetSystemLibrary.PrintString` "swap")
  (if (> (`KismetArrayLibrary.Array_Length` (`self.PlayerRef`)) 1)
    (bind _outhit (`KismetSystemLibrary.SphereTraceSingle_NEW` :`End` (0.0 0.0 111.0) :`Radius` 4440.0 :`TraceChannel` "TraceTypeQuery1" :`bTraceComplex` true :`DrawDebugType` "ForOneFrame"))
    (for _index (range (`KismetArrayLibrary.Array_Length` _playerref))
      (bind (_bblockinghit _time _location _normal _impactpoint _impactnormal _physmat _hitactor) (`GameplayStatics.BreakHitResult` _outhit))
      (if (== _hitactor (`KismetArrayLibrary.Array_Get` _playerref _index))
        (if (!= _hitactor (`BlackboardComponent.GetValueAsObject` _returnvalue _enemyactor))
          (break))))
    (`BlackboardComponent.SetValueAsObject` _returnvalue _enemyactor _hitactor)))

(fn `UserConstructionScript`
  (`parent.UserConstructionScript`))