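; AI_Boss1_Plot is a boss AI Blueprint that launches a fire wave attack when its enemy-found event fires.
; EnemyFoundEvent waits briefly, then spawns a WaveAttackFire actor ahead along the control rotation, lowered from the boss's origin and using the actor's rotation.
; The attack runs once per event through a single-branch Sequence; BeginPlay, overlap, Tick and construction add no logic of their own.
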(event `self.ReceiveBeginPlay`
  (`parent.ReceiveBeginPlay`))

(event `self.ReceiveActorBeginOverlap`
  (params (OtherActor :type "Actor Object Reference")))

(event `self.EnemyFound_Event`
  (`|ExecutionSequence`
    (:`then_0`
      ;[1 1 1] Attack 1
      (`KismetSystemLibrary.Delay` 1.0)
      (`|SpawnActorFromClass` "/Game/Blueprints/bossattacks/WaveAttackFire.WaveAttackFire_C" (`KismetMathLibrary.MakeTransform` (- (+ (`self.K2_GetActorLocation`) (* (`KismetMathLibrary.GetForwardVector` (`self.GetControlRotation`)) 200.0)) (0.0 0.0 90.0)) (`self.K2_GetActorRotation`) (1.0 1.0 1.0))))))

(event `self.ReceiveTick`
  (params (DeltaSeconds :type "Float (single-precision)"))
  (`parent.ReceiveTick` 0.0))

(fn `UserConstructionScript`
  (`parent.UserConstructionScript`))