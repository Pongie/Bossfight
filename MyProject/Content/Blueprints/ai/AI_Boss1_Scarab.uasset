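; Scarab boss AI pawn that attacks players when its EnemyFound event fires, also spawning an omnidirectional attack actor at BeginPlay.
; One sequence runs cooldown-gated melee with move-to, randomly rolled homing missiles using a line trace and custom-depth target highlight, and a random burrow that hides, spawns Burrow_Attack, then reappears.
; BeginPlay starts a looping AggroSwap timer, but the aggro-swap logic here is disconnected.
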(event `self.ReceiveBeginPlay`
  ;[1 1 1] init
  (`parent.ReceiveBeginPlay`)
  (cast `/Game/Blueprints/MyGameInstance` (`GameplayStatics.GetGameInstance`))
  (bind _asai_boss_pat (cast `/Game/Blueprints/ai/AI_Boss_Pat` (`self.GetController`)))
  (cast `/Game/Blueprints/ai/AI_Boss1` (`Controller.K2_GetPawn` _asai_boss_pat))
  (`KismetSystemLibrary.K2_SetTimer` null "AggroSwap" (`KismetMathLibrary.RandomFloatInRange` 7.0 17.0) true)
  (`|SpawnActorFromClass` "/Game/Blueprints/bossattacks/Omnidirection_attack.Omnidirection_attack_C" (`KismetMathLibrary.MakeTransform` (0.0 0.0 0.0)) true self))

(event `EnemyFound_Event`
  (bind _returnvalue (`SceneComponent.K2_GetComponentLocation`))
  (bind _homingtarget (`self.HomingTarget`))
  (bind _item (`KismetArrayLibrary.Array_Get` (`self.GetOverlappingActors` "/Game/Blueprints/MyCharacter.MyCharacter_C")))
  (bind _location (.location (`self.GetTransform`)))
  (bind _rotation (.rotation (`self.GetTransform`)))
  (bind _returnvalue_2 (* (`KismetMathLibrary.Conv_RotatorToVector` _rotation) 900.0))
  ;[1 1 1] Attack sequence
  (`|ExecutionSequence`
    (:`then_0`
      ;[1 1 1] Melee
      (if (not (!= _item null)) :!label _label
        (`|AIMoveTo` self (`self.K2_GetActorLocation` _item) _item 2.0
          (:`OnSuccess`
            _)
          (:`OnFail`
            (goto _label))))
      (`/Engine/EditorBlueprintResources/StandardMacros.CompareFloat` (`self.coolDownM`) (`KismetSystemLibrary.GetGameTimeInSeconds`)
        (:`<`
          (`SkeletalMeshComponent.PlayAnimation` (`self.Mesh`) "/Game/Outsourced/Meshes/Mixamo_Maw/Anims/Maw_J_Laygo_Sword_Swing.Maw_J_Laygo_Sword_Swing" false)
          (`GameplayStatics.ApplyDamage` (`KismetArrayLibrary.Array_Get` (`PrimitiveComponent.GetOverlappingActors` (`self.MeleeRange`) "/Game/Blueprints/MyCharacter.MyCharacter_C")) 6.0)
          (set `self.coolDownM` (+ (`KismetSystemLibrary.GetGameTimeInSeconds`) 0.8))
          (if (>= (`KismetMathLibrary.RandomFloatInRange` 0.0 100.0) 50.0)
            (`KismetSystemLibrary.Delay` 0.2)
            (goto _label)))))
    (:`then_1`
      ;[1 1 1] Homing Missle
      (`KismetSystemLibrary.Delay` 0.2)
      (if (>= (`KismetMathLibrary.RandomFloatInRange` 0.0 100.0) 70.0)
        (bind (_outhit _returnvalue_3) (`KismetSystemLibrary.LineTraceSingleForObjects` (`KismetMathLibrary.MakeVector` (.x _returnvalue) (.y _returnvalue) (- (.z _returnvalue) 390.0)) (`KismetMathLibrary.MakeVector` (.x (+ (* (`KismetMathLibrary.GetForwardVector` (.rotation (`SceneComponent.K2_GetComponentToWorld`))) 3330.0) _returnvalue)) (.y (+ (* (`KismetMathLibrary.GetForwardVector` (.rotation (`SceneComponent.K2_GetComponentToWorld`))) 3330.0) _returnvalue)) (- (.z (+ (* (`KismetMathLibrary.GetForwardVector` (.rotation (`SceneComponent.K2_GetComponentToWorld`))) 3330.0) _returnvalue)) 390.0)) (`self.ObjectsToTarget`) true))
        ;;[1 1 1] Taargeting for missle
        (if _returnvalue_3
          (bind _asmy_character (cast `/Game/Blueprints/MyCharacter` (`.HitActor` (`GameplayStatics.BreakHitResult` _outhit))))
          (`/Engine/EditorBlueprintResources/StandardMacros.IsValid` _homingtarget
            (:`Is Valid`
              (`PrimitiveComponent.SetRenderCustomDepth` _homingtarget false))
            (:`Is Not Valid`
              _))
          (bind _output_get (set `self.HomingTarget` (`Character.CapsuleComponent` _asmy_character)))
          (`PrimitiveComponent.SetRenderCustomDepth` _homingtarget true)
          (`PrimitiveComponent.SetRenderCustomDepth` _output_get true)
          (else
            (`/Engine/EditorBlueprintResources/StandardMacros.IsValid` _homingtarget
              (:`Is Valid`
                (`PrimitiveComponent.SetRenderCustomDepth` _homingtarget true)))))
        (bind _returnvalue_4 (`|SpawnActorFromClass` "/Game/Blueprints/bossattacks/homing_attack.homing_attack_C" (`KismetMathLibrary.MakeTransform` (- (+ (`self.K2_GetActorLocation`) (* (`KismetMathLibrary.GetForwardVector` (`self.GetControlRotation`)) 400.0)) (0.0 0.0 190.0)) (`self.K2_GetActorRotation`) (1.0 1.0 1.0)) true))
        (`/Game/Blueprints/bossattacks/homing_attack.Homing Missle` _returnvalue_4 (`self.HomingTarget`))))
    (:`then_2`
      ;[1 1 1] Burrow Attack
      (`KismetSystemLibrary.PrintString` "Burrow")
      (if (>= (`KismetMathLibrary.RandomFloatInRange` 0.0 100.0) 40.0)
        (if (not (`self.Inburrow`))
          (set `self.Inburrow` true)
          (bind _outhits (`KismetSystemLibrary.BoxTraceMulti` _location _returnvalue_2 (600.0 600.0 120.0) (struct) "TraceTypeQuery1" true))
          (for _array_element _outhits
            (cast `/Game/Blueprints/MyCharacter` (`.HitActor` (`GameplayStatics.BreakHitResult` _array_element)))
            (`/Engine/EditorBlueprintResources/StandardMacros.DoOnce` false :!label _label_2
              (:`Completed`
                (set `self.intialZlocation` _location)
                (`SceneComponent.SetHiddenInGame` true)
                (`|SpawnActorFromClass` "/Game/Blueprints/bossattacks/Burrow_Attack.Burrow_Attack_C" (`KismetMathLibrary.MakeTransform` (- _location (0.0 0.0 420.0)) _rotation) true)
                (`KismetSystemLibrary.Delay` 1.7)
                (`self.K2_SetActorTransform` (`KismetMathLibrary.MakeTransform` (+ _returnvalue_2 (0.0 0.0 530.0)) _rotation (4.25 4.25 4.25)))
                (`SceneComponent.SetHiddenInGame` false)
                (set `self.Inburrow` false))))
          (goto _label_2 :!via `Reset`)
          (else
            (bind _outactors (`GameplayStatics.GetAllActorsOfClass` "/Game/Blueprints/bossattacks/Burrow_Attack.Burrow_Attack_C"))
            (if (== (`KismetArrayLibrary.Array_Get` _outactors) null)
              (set `self.Inburrow` false))))))))

(event `self.ReceiveActorBeginOverlap`
  (params (OtherActor :type "Actor Object Reference")))

(event `self.ReceiveTick`
  (params (DeltaSeconds :type "Float (single-precision)"))
  (`parent.ReceiveTick` 0.0))

(fn `UserConstructionScript`
  (`parent.UserConstructionScript`))