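; Rotating wall hazard tied to the AI_Boss1 boss that damages the player on contact.
; On BeginPlay it casts BossRef to AI_Boss1, sets the RotatingMovement pivot translation to the boss's world location with local-space rotation, and re-sets the boss to its current location.
; Cube overlaps apply a small fixed damage to MyCharacter actors.
; The construction script holds only an unconnected copy of the pivot setup.
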(event `self.ReceiveTick`
  (params (DeltaSeconds :type "Float (single-precision)")))

(event `self.ReceiveActorBeginOverlap`
  (params (OtherActor :type "Actor Object Reference")))

(event `self.ReceiveBeginPlay`
  (bind _rotatingmovement (`self.RotatingMovement`))
  ;[1 1 1] Initialize
  (bind _asai_boss_1 (cast `/Game/Blueprints/ai/AI_Boss1` (`self.BossRef`)))
  (bind _returnvalue (`SceneComponent.K2_GetComponentLocation` _asai_boss_1))
  (set `RotatingMovementComponent.PivotTranslation` _returnvalue _rotatingmovement)
  (set `RotatingMovementComponent.bRotationInLocalSpace` true _rotatingmovement)
  (`self.K2_SetActorLocation` _asai_boss_1 _returnvalue false))

(event `self.Cube.OnComponentBeginOverlap`
  (params (OtherActor :type "Actor Object Reference") (OtherComp :type "PrimitiveComponent Object Reference") (OtherBodyIndex :type Integer) (bFromSweep :type Boolean) (SweepResult :type "EngineTypes.HitResult Structure (by ref)"))
  ;[1 1 1] Damage
  (if (`KismetMathLibrary.ClassIsChildOf` (`GameplayStatics.GetObjectClass` OtherActor) "/Game/Blueprints/MyCharacter.MyCharacter_C")
    (`GameplayStatics.ApplyDamage` OtherActor 3.0)))

(fn `UserConstructionScript`)