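; AgroCheck is a behavior tree node that looks for targets around a follower AI on each tick.
; It caches the Follower_AI_CON controller, then sphere-traces around the pawn for configured object types, ignoring all AI_character actors.
; A camera-channel line trace checks sight to each hit, writing TargetToFollow and TargetLocation when clear and clearing only TargetToFollow when blocked.
; Each hit overwrites the previous result, so the last one decides.
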(event `self.ReceiveTick`
  (params (OwnerActor :type "Actor Object Reference") (DeltaSeconds :type "Float (single-precision)"))
  (bind _targettofollow (`self.TargetToFollow`))
  (if (not (!= (`self.Ai Controller Ref`) null))
    (bind _asfollower_ai_con (cast `/Game/Blueprints/ai/FOLLOWER_AI_CON` OwnerActor))
    (bind _output_get (set `self.Ai Controller Ref` _asfollower_ai_con)))
  (bind _outactors (`GameplayStatics.GetAllActorsOfClass` "/Game/Blueprints/ai/ai_character.AI_character_C"))
  (bind _returnvalue (`Actor.K2_GetActorLocation` (`Controller.K2_GetPawn` _output_get)))
  (set `self.MyLocation` _returnvalue)
  (bind _outhits (`KismetSystemLibrary.SphereTraceMultiForObjects` _returnvalue (+ _returnvalue (0.0 0.0 15.0)) 1500.0 (`self.DesiredObjectType`) false _outactors))
  (for _array_element _outhits
    (bind (_bblockinghit _time _location _normal _impactpoint _impactnormal _physmat _hitactor) (`GameplayStatics.BreakHitResult` _array_element))
    (bind _outhit (`KismetSystemLibrary.LineTraceSingle` (`self.MyLocation`) (`Actor.K2_GetActorLocation` _hitactor) "TraceTypeQuery2" false _outactors))
    (bind (_bblockinghit_2 _time_2 _location_2 _normal_2 _impactpoint_2 _impactnormal_2 _physmat_2 _hitactor_2) (`GameplayStatics.BreakHitResult` _outhit))
    (if (== _hitactor_2 _hitactor)
      (`BTFunctionLibrary.SetBlackboardValueAsObject` _targettofollow _hitactor_2)
      (`BTFunctionLibrary.SetBlackboardValueAsVector` (`self.TargetLocation`) (`Actor.K2_GetActorLocation` _hitactor_2))
      (else
        (`BTFunctionLibrary.SetBlackboardValueAsObject` _targettofollow)))))