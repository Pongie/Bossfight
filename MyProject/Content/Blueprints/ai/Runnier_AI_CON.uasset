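; AI controller for the Runnier enemy that runs the RunnerBT behavior tree and tracks the player as its target.
; One second after BeginPlay, SetEnemy stores the first player pawn and writes it to the Blackboard's player key when it changes.
; Perception updates matching that pawn set the player-visible key to true; the sight check is unfinished, so the flag is never cleared here.
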(event `self.AIPerception.OnPerceptionUpdated`
  (params (UpdatedActors :type "Array of Actor Object Reference"))
  (for _array_element UpdatedActors
    (if (== _array_element (`self.Player(Enemy)`))
      (bind _info (`AIPerceptionComponent.GetActorsPerception` (`self.AIPerception`) _array_element))
      (`BlackboardComponent.SetValueAsBool` (`AIBlueprintHelperLibrary.GetBlackboard` null) (`self.BlackboardKeyIsPlayerVisible`) true) ; the logic for this is in 4.8, for now i have no idea what the condition grab is called for sensing if a player is visible, and this will always be true, so the thing should alway act as if visible
    )))

(event `self.ReceiveBeginPlay`
  (`self.RunBehaviorTree` "/Game/Blueprints/ai/RunnerBT.RunnerBT")
  (`KismetSystemLibrary.Delay` 1.0)
  (`self.SetEnemy` (`GameplayStatics.GetPlayerPawn` 0)))

(event `self.ReceiveTick`
  (params (DeltaSeconds :type "Float (single-precision)")))

(fn `SetEnemy`
  (params (NewEnemy :type "Actor Object Reference"))
  (if (!= NewEnemy (`self.Player(Enemy)`))
    (bind _output_get (set `self.Player(Enemy)` NewEnemy))
    (`BlackboardComponent.SetValueAsObject` (`AIBlueprintHelperLibrary.GetBlackboard` null) (`self.BlackboardKeyPlayer`) _output_get)))

(fn `UserConstructionScript`)