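; Spear weapon Blueprint whose primary attack spawns a short-lived, scaled-down Lion_Burst just in front of the player, facing the player's rotation.
; Attack1 rate-limits itself by comparing a stored cooldown timestamp against game time.
; Attack2 and Attack3 are empty stubs returning false.
; BeginPlay casts the player to MyCharacter, but the logic toggling spear mesh visibility from Spearequipped is disconnected and never runs.
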(event `self.ReceiveBeginPlay`
  (bind _asmy_character (cast `/Game/Blueprints/MyCharacter` (`GameplayStatics.GetPlayerCharacter` 0))
    (:`CastFailed`
      (`KismetSystemLibrary.PrintString` "?"))))

(event `self.ReceiveActorBeginOverlap`
  (params (OtherActor :type "Actor Object Reference")))

(event `self.ReceiveTick`
  (params (DeltaSeconds :type "Float (single-precision)")))

(fn `Attack1`
  (returns (NewParam :type Boolean))
  (bind _myplayer (`self.myPlayer`))
  (bind _returnvalue (`self.K2_GetActorRotation` _myplayer))
  (`/Engine/EditorBlueprintResources/StandardMacros.CompareFloat` (`self.CoolDown1`) (`KismetSystemLibrary.GetGameTimeInSeconds`)
    (:`<`
      (bind _returnvalue_2 (`|SpawnActorFromClass` "/Game/Blueprints/Lion_Burst.Lion_Burst_C" (`KismetMathLibrary.MakeTransform` (+ (`self.K2_GetActorLocation` _myplayer) (* (`KismetMathLibrary.GetForwardVector` _returnvalue) 100.0)) _returnvalue (0.3 0.3 0.3))))
      (`self.SetLifeSpan` _returnvalue_2 0.75)
      (set `self.CoolDown1` (+ (`KismetSystemLibrary.GetGameTimeInSeconds`) 0.5))
      (return false))))

(fn `Attack2`
  (returns (NewParam :type Boolean))
  (return false))

(fn `Attack3`
  (returns (NewParam :type Boolean))
  (return false))

(fn `UserConstructionScript`
  (`parent.UserConstructionScript`))