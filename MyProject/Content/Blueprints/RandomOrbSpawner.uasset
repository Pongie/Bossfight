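; RandomOrbSpawner is an actor that spawns a Fire, Water or Wind orb at its Sphere component's transform.
; BeginPlay casts House3_BP to RandomOrbSpawner and binds to its Dothething dispatcher, printing a debug string if the cast fails.
; The bound event picks the class from CurrentOrb and spawns it even if colliding.
; RandomOrb randomizes CurrentOrb, but nothing in this Blueprint calls it.
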(event `self.ReceiveBeginPlay`
  (bind _asrandom_orb_spawner (castclass `/Game/Blueprints/RandomOrbSpawner` "/Game/Blueprints/House3_BP.House3_BP_C")
    (:`then`
      (`GameplayStatics.GetAllActorsOfClass` _asrandom_orb_spawner)
      (add `self.dothething` (delegate `dothething_Event`)))
    (:`CastFailed`
      (`KismetSystemLibrary.PrintString` "ddddd"))))

(event `dothething_Event` :!signature `self.dothething`
  (params (NewParam :type Boolean))
  (bind _returnvalue (`SceneComponent.K2_GetComponentToWorld` (`self.Sphere`)))
  (if (== (`self.CurrentOrb`) 0)
    (`|SpawnActorFromClass` "/Game/Blueprints/Fire.Fire_C" _returnvalue true)
    (elif (== (`self.CurrentOrb`) 1)
      (`|SpawnActorFromClass` "/Game/Blueprints/Water.Water_C" _returnvalue true)
      (elif (== (`self.CurrentOrb`) 2)
        (`|SpawnActorFromClass` "/Game/Blueprints/Wind.Wind_C" _returnvalue true)))))

(event `self.ReceiveActorBeginOverlap`
  (params (OtherActor :type "Actor Object Reference")))

(event `self.ReceiveTick`
  (params (DeltaSeconds :type "Float (single-precision)")))

(fn `RandomOrb`
  (set `self.CurrentOrb` (`KismetMathLibrary.RandomIntegerInRange` 0 2)))

(fn `UserConstructionScript`)