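; Spawner actor that places two random elemental orbs in the world when play begins.
; Each orb is an independent random pick of Fire, Water, Wind or Aether, so both can share a type.
; Spawn points are random in X and Y within the Box component's scaled extent, at the height of its top, offset from the actor's location.
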(event `self.ReceiveBeginPlay`
  (bind _x (.x (`BoxComponent.GetScaledBoxExtent` (`self.Box`))))
  (bind _y (.y (`BoxComponent.GetScaledBoxExtent` (`self.Box`))))
  (bind _returnvalue (`KismetMathLibrary.Conv_VectorToTransform` (+ (`KismetMathLibrary.MakeVector` (`KismetMathLibrary.RandomFloatInRange` (* _x -1.0) _x) (`KismetMathLibrary.RandomFloatInRange` (* _y -1.0) _y) (.z (`BoxComponent.GetScaledBoxExtent` (`self.Box`)))) (`self.K2_GetActorLocation`))))
  ;[1 1 1] Orb 1 spawn
  (bind _output_get (set `self.CurrentOrb` (`KismetMathLibrary.RandomIntegerInRange` 0 3)))
  (switch `int` _output_get
    (:`0`
      (`|SpawnActorFromClass` "/Game/Blueprints/Items/Fire.Fire_C" _returnvalue))
    (:`1`
      (`|SpawnActorFromClass` "/Game/Blueprints/Items/Water.Water_C" _returnvalue))
    (:`2`
      (`|SpawnActorFromClass` "/Game/Blueprints/Items/Wind.Wind_C" _returnvalue))
    (:`3`
      (`|SpawnActorFromClass` "/Game/Blueprints/Items/Aether.Aether_C" _returnvalue)))
  ;[1 1 1] Orb 2 spawn
  (bind _output_get_2 (set `self.CurrentOrb` (`KismetMathLibrary.RandomIntegerInRange` 0 3)))
  (switch `int` _output_get_2
    (:`0`
      (`|SpawnActorFromClass` "/Game/Blueprints/Items/Fire.Fire_C" _returnvalue))
    (:`1`
      (`|SpawnActorFromClass` "/Game/Blueprints/Items/Water.Water_C" _returnvalue))
    (:`2`
      (`|SpawnActorFromClass` "/Game/Blueprints/Items/Wind.Wind_C" _returnvalue))
    (:`3`
      (`|SpawnActorFromClass` "/Game/Blueprints/Items/Aether.Aether_C" _returnvalue))))

(fn `UserConstructionScript`)