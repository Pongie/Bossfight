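; MySave is a Blueprint that saves and loads basic player data (HP, name, slot, index) with hardcoded test values.
; Save sets those fields, then writes SaveInstance to disk using that instance's slot name and index.
; Load reads the fixed Slot0, casts it to MySave, stores it as SaveInstance and prints the saved name.
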(fn `Load`
  (bind _returnvalue (`GameplayStatics.LoadGameFromSlot` "Slot0"))
  (bind _asmy_save (cast `/Game/Blueprints/MySave` _returnvalue))
  (bind _output_get (set `self.SaveInstance` _asmy_save))
  (`KismetSystemLibrary.PrintString` null (`/Game/Blueprints/MySave.Name` _output_get)))

(fn `Save`
  (bind _saveinstance (`self.SaveInstance`))
  (set `self.HP` 50)
  (set `self.Name` "BananaCrab")
  (set `self.SlotName` "Slot0")
  (set `self.Index` 0)
  (`GameplayStatics.SaveGameToSlot` _saveinstance (`/Game/Blueprints/MySave.SlotName` _saveinstance) (`/Game/Blueprints/MySave.Index` _saveinstance)))