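; Game instance that carries each player's orbs and utilities between spawns and saves progress to per-player slots.
; Saving flattens equipped and inventory items into name, level and count structs in memory, then writes only the active orb and boss progress to MySave slots.
; Loading respawns items as hidden, non-colliding actors and refills inventory and UI.
; On first spawn the orb comes from the slot file, or a new save is created.
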(fn `ItemToStruct`
  (params (self2 :type "/Game/Blueprints/Items/Item Object Reference"))
  (returns (ItemStruct :type "/Game/Blueprints/ItemStruct Structure"))
  (return (make `/Game/Blueprints/ItemStruct` (`/Game/Blueprints/Items/Item.name` self2) (`/Game/Blueprints/Items/Item.level` self2) (`/Game/Blueprints/Items/Item.count` self2))))

(fn `LoadPlayerCharacter`
  (params (player :type "/Game/Blueprints/MyCharacter Object Reference"))
  (bind _inventorydisplay (`/Game/Blueprints/MyCharacter.InventoryDisplay` player))
  (bind (_equippedorb _orbinventory _utilityinventory _utility1 _utility2 _utility3) (break `/Game/Blueprints/PlayerStruct` (`KismetArrayLibrary.Array_Get` (`self.playerItems`) (`/Game/Blueprints/MyCharacter.playerNum` player))))
  (if (`self.firstSpawn`)
    (`self.LoadPlayerFromFile` player)
    (else
      (bind _resultitem (`self.StructToItem` player _equippedorb))
      (`/Engine/EditorBlueprintResources/StandardMacros.IsValid` _resultitem
        (:`Is Valid`
          (bind _asorb (cast `/Game/Blueprints/Items/Orb` _resultitem))
          (bind _output_get (set `/Game/Blueprints/MyCharacter.activeOrb` _asorb player))
          (`/Game/Blueprints/Items/Orb.orbifyPlayer` _output_get player)
          (set `/Game/Blueprints/Widgets/OrbEquip.myItem` _output_get (`/Game/Blueprints/Widgets/InventoryScreen.EquippedOrb` _inventorydisplay)))
        (:`Is Not Valid`
          _))))
  (bind _resultitem_2 (`self.StructToItem` player _utility1))
  (`/Engine/EditorBlueprintResources/StandardMacros.IsValid` _resultitem_2
    (:`Is Valid`
      (bind _asutility (cast `/Game/Blueprints/Items/Utility` _resultitem_2)
        (:`then`
          (bind _output_get_2 (set `/Game/Blueprints/MyCharacter.Utility1` _asutility player))
          (set `/Game/Blueprints/Widgets/ItemSlot.myItem` _output_get_2 (`/Game/Blueprints/Widgets/InventoryScreen.EquippedUtility1` _inventorydisplay)))
        (:`CastFailed`
          _)))
    (:`Is Not Valid`
      _))
  (bind _resultitem_3 (`self.StructToItem` player _utility2))
  (`/Engine/EditorBlueprintResources/StandardMacros.IsValid` _resultitem_3
    (:`Is Valid`
      (bind _asutility_2 (cast `/Game/Blueprints/Items/Utility` _resultitem_3)
        (:`then`
          (bind _output_get_3 (set `/Game/Blueprints/MyCharacter.Utility2` _asutility_2 player))
          (set `/Game/Blueprints/Widgets/ItemSlot.myItem` _output_get_3 (`/Game/Blueprints/Widgets/InventoryScreen.EquippedUtility2` _inventorydisplay)))
        (:`CastFailed`
          _)))
    (:`Is Not Valid`
      _))
  (bind _resultitem_4 (`self.StructToItem` player _utility3))
  (`/Engine/EditorBlueprintResources/StandardMacros.IsValid` _resultitem_4
    (:`Is Valid`
      (bind _asutility_3 (cast `/Game/Blueprints/Items/Utility` _resultitem_4)
        (:`then`
          (bind _output_get_4 (set `/Game/Blueprints/MyCharacter.Utility3` _asutility_3 player))
          (set `/Game/Blueprints/Widgets/ItemSlot.myItem` _output_get_4 (`/Game/Blueprints/Widgets/InventoryScreen.EquippedUtility3` _inventorydisplay)))
        (:`CastFailed`
          _)))
    (:`Is Not Valid`
      _))
  (`self.StructToOrbList` player _orbinventory)
  (`self.StructToUtilityList` player _utilityinventory))

(fn `LoadPlayerFromFile`
  (params (player :type "/Game/Blueprints/MyCharacter Object Reference"))
  (bind _playernum (`/Game/Blueprints/MyCharacter.playerNum` player))
  (bind _returnvalue (`KismetStringLibrary.Conv_IntToString` (`KismetArrayLibrary.Array_Get` (`self.playerSaveSlotChoices`) _playernum)))
  (bind _returnvalue_2 (`GameplayStatics.DoesSaveGameExist` _returnvalue))
  (if (and _returnvalue_2 (`KismetArrayLibrary.Array_Get` (`self.isPlayerLoading`) _playernum))
    (bind _returnvalue_3 (`GameplayStatics.LoadGameFromSlot` _returnvalue))
    (bind _asmy_save (cast `/Game/Blueprints/MySave` _returnvalue_3))
    (`self.StructToItem` player (`/Game/Blueprints/MySave.savedOrb` _asmy_save))
    (bind _asorb (cast `/Game/Blueprints/Items/Orb` null))
    (bind _output_get (set `/Game/Blueprints/MyCharacter.activeOrb` _asorb player))
    (set `/Game/Blueprints/Widgets/OrbEquip.myItem` _output_get (`/Game/Blueprints/Widgets/InventoryScreen.EquippedOrb` (`/Game/Blueprints/MyCharacter.InventoryDisplay` player)))
    (`KismetArrayLibrary.Array_Add` (`self.playerExternalSaves`) _asmy_save)
    (`KismetSystemLibrary.PrintString` "loaded")
    (else
      (bind _returnvalue_4 (`GameplayStatics.CreateSaveGameObject` "/Game/Blueprints/MySave.MySave_C"))
      (bind _asmy_save_2 (cast `/Game/Blueprints/MySave` _returnvalue_4))
      (`KismetArrayLibrary.Array_Add` (`self.playerExternalSaves`) _asmy_save_2)
      (`KismetSystemLibrary.PrintString` "did not load"))))

(fn `OrbListToStruct`
  (params (playerNum :type Integer :default 0) (NewParam1 :type "Array of /Game/Blueprints/ItemStruct Structure"))
  (returns (NewParam :type "Array of /Game/Blueprints/ItemStruct Structure"))
  (bind _asmy_character (cast `/Game/Blueprints/MyCharacter` (`GameplayStatics.GetPlayerCharacter` playerNum)))
  (bind _orblist (`/Game/Blueprints/Inventory.orbList` (`/Game/Blueprints/MyCharacter.Inventory` _asmy_character)))
  (for _index (range (+ (`KismetArrayLibrary.Array_LastIndex` _orblist) 1))
    (bind _itemstruct (`self.ItemToStruct` (`KismetArrayLibrary.Array_Get` _orblist _index)))
    (`KismetArrayLibrary.Array_Add` NewParam1 _itemstruct))
  (return NewParam1))

(fn `SavePlayerCharacters`
  (bind _playeritems (`self.playerItems`))
  (`KismetArrayLibrary.Array_Clear` _playeritems)
  (for _index (range (`self.playerCount`))
    (bind _asmy_character (cast `/Game/Blueprints/MyCharacter` (`GameplayStatics.GetPlayerCharacter` _index)))
    (bind _activeorb (`/Game/Blueprints/MyCharacter.activeOrb` _asmy_character))
    (`/Engine/EditorBlueprintResources/StandardMacros.IsValid` _activeorb
      (:`Is Valid`
        (bind _itemstruct (`self.ItemToStruct` _activeorb)))
      (:`Is Not Valid`
        _))
    (bind (_equippedorb _orbinventory _utilityinventory) (break `/Game/Blueprints/PlayerStruct` (`KismetArrayLibrary.Array_Get` _playeritems _index)))
    (bind _newparam (`self.OrbListToStruct` _index _orbinventory))
    (bind _newparam_2 (`self.UtilityListToStruct` _index _utilityinventory))
    (bind _utility1 (`/Game/Blueprints/MyCharacter.Utility1` _asmy_character))
    (`/Engine/EditorBlueprintResources/StandardMacros.IsValid` _utility1
      (:`Is Valid`
        (bind _itemstruct_2 (`self.ItemToStruct` _utility1)))
      (:`Is Not Valid`
        _))
    (bind _utility2 (`/Game/Blueprints/MyCharacter.Utility2` _asmy_character))
    (`/Engine/EditorBlueprintResources/StandardMacros.IsValid` _utility2
      (:`Is Valid`
        (bind _itemstruct_3 (`self.ItemToStruct` _utility2))
        (bind _utility3 (`/Game/Blueprints/MyCharacter.Utility3` _asmy_character))
        (bind _itemstruct_4 (`self.ItemToStruct` _utility3 :!label _label)))
      (:`Is Not Valid`
        (`/Engine/EditorBlueprintResources/StandardMacros.IsValid` _utility3
          (:`Is Valid`
            (goto _label))
          (:`Is Not Valid`
            _))))
    (`KismetArrayLibrary.Array_Add` _playeritems (make `/Game/Blueprints/PlayerStruct` _itemstruct _newparam _newparam_2 _itemstruct_2 _itemstruct_3 _itemstruct_4)))
  (`self.SavePlayersToFile`))

(fn `SavePlayersToFile`
  (for _index (range (`self.playerCount`))
    (bind _asmy_character (cast `/Game/Blueprints/MyCharacter` (`GameplayStatics.GetPlayerCharacter` _index)))
    (bind _itemstruct (`self.ItemToStruct` (`/Game/Blueprints/MyCharacter.activeOrb` _asmy_character)))
    (bind _playernum (`/Game/Blueprints/MyCharacter.playerNum` _asmy_character))
    (bind _item (`KismetArrayLibrary.Array_Get` (`self.playerExternalSaves`) _playernum))
    (set `/Game/Blueprints/MySave.savedOrb` _itemstruct _item)
    (set `/Game/Blueprints/MySave.bossesKilled` (`self.bossesDefeated`) _item)
    (set `/Game/Blueprints/MySave.lastBossKillTime` 0.0 _item)
    (`GameplayStatics.SaveGameToSlot` _item (`KismetStringLibrary.Conv_IntToString` (`KismetArrayLibrary.Array_Get` (`self.playerSaveSlotChoices`) _playernum)))))

(fn `StructToItem`
  (params (character :type "/Game/Blueprints/MyCharacter Object Reference") (item :type "/Game/Blueprints/ItemStruct Structure"))
  (returns (resultItem :type "/Game/Blueprints/Items/Item Object Reference"))
  (bind (_name _level _count) (break `/Game/Blueprints/ItemStruct` item))
  (bind _result (`/Game/Blueprints/MyCharacter.result` character))
  (`/Game/Blueprints/MyCharacter.SpawnItem` character _name)
  (`PrimitiveComponent.SetSimulatePhysics` _result false)
  (`PrimitiveComponent.SetCollisionEnabled` _result "NoCollision")
  (`SceneComponent.SetVisibility` _result false true)
  (set `/Game/Blueprints/Items/Item.level` _level _result)
  (set `/Game/Blueprints/Items/Item.count` _count _result)
  (return _result))

(fn `StructToOrbList`
  (params (player :type "/Game/Blueprints/MyCharacter Object Reference") (structList :type "Array of /Game/Blueprints/ItemStruct Structure"))
  (for _index (range (+ (`KismetArrayLibrary.Array_LastIndex` structList) 1))
    (bind _resultitem (`self.StructToItem` player (`KismetArrayLibrary.Array_Get` structList _index)))
    (bind _asorb (cast `/Game/Blueprints/Items/Orb` _resultitem))
    (`KismetArrayLibrary.Array_Add` (`/Game/Blueprints/Inventory.orbList` (`/Game/Blueprints/MyCharacter.Inventory` player)) _asorb)))

(fn `StructToUtilityList`
  (params (player :type "/Game/Blueprints/MyCharacter Object Reference") (structList :type "Array of /Game/Blueprints/ItemStruct Structure"))
  (for _index (range (+ (`KismetArrayLibrary.Array_LastIndex` structList) 1))
    (bind _item (`KismetArrayLibrary.Array_Get` structList _index))
    (`KismetSystemLibrary.PrintString` (`.name_9_9E9CFFA3466813D03A9851881A570BE9` (break `/Game/Blueprints/ItemStruct` _item)))
    (bind _resultitem (`self.StructToItem` player _item))
    (bind _asutility (cast `/Game/Blueprints/Items/Utility` _resultitem))
    (`KismetArrayLibrary.Array_Add` (`/Game/Blueprints/Inventory.utilityList` (`/Game/Blueprints/MyCharacter.Inventory` player)) _asutility)))

(fn `UtilityListToStruct`
  (params (playerNum :type Integer :default 0) (NewParam1 :type "Array of /Game/Blueprints/ItemStruct Structure"))
  (returns (NewParam :type "Array of /Game/Blueprints/ItemStruct Structure"))
  (bind _asmy_character (cast `/Game/Blueprints/MyCharacter` (`GameplayStatics.GetPlayerCharacter` playerNum)))
  (bind _utilitylist (`/Game/Blueprints/Inventory.utilityList` (`/Game/Blueprints/MyCharacter.Inventory` _asmy_character)))
  (for _index (range (+ (`KismetArrayLibrary.Array_LastIndex` _utilitylist) 1))
    (bind _itemstruct (`self.ItemToStruct` (`KismetArrayLibrary.Array_Get` _utilitylist _index)))
    (`KismetArrayLibrary.Array_Add` NewParam1 _itemstruct))
  (return NewParam1))