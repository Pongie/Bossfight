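; Potion Blueprint, a consumable item that restores health to the player character.
; Use casts the given player to MyCharacter, adds PotionPoints to CurrentHealth with no clamping, then destroys the potion and returns false.
; The event graph holds only disabled default events, and the construction script just calls its parent.
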(event `self.ReceiveBeginPlay`)

(event `self.ReceiveActorBeginOverlap`
  (params (OtherActor :type "Actor Object Reference"))
  (`parent.ReceiveActorBeginOverlap` null))

(event `self.ReceiveTick`
  (params (DeltaSeconds :type "Float (single-precision)")))

(fn `Use`
  (params (Player :type "/Game/Blueprints/MyCharacter Object Reference"))
  (returns (NewParam :type Boolean))
  (bind _asmy_character (cast `/Game/Blueprints/MyCharacter` Player))
  (set `/Game/Blueprints/MyCharacter.CurrentHealth` (+ (`/Game/Blueprints/MyCharacter.CurrentHealth` _asmy_character) (`self.potionPoints`)) _asmy_character)
  (`self.K2_DestroyActor`)
  (return false))

(fn `UserConstructionScript`
  (`parent.UserConstructionScript`))